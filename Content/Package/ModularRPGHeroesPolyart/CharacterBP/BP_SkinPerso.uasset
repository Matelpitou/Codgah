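; Modular RPG hero character Blueprint that assembles a skinned character from separate body, armor and equipment mesh components.
; On BeginPlay, UpdateSkin sets the main skeletal mesh as leader pose for hair, face and worn armor pieces so they animate together.
; UpdateOutline toggles render custom depth on the body, all those pieces, weapons, shield and backpack, apparently for an outline effect.
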(event `self.ReceiveBeginPlay`
  (`self.UpdateSkin`))

(fn `UpdateOutline`
  (params (`Visible?` :type Boolean))
  (locals (`LVisible?` :type Boolean))
  (set `local.LVisible?` `Visible?`)
  (`PrimitiveComponent.SetRenderCustomDepth` (`self.SkeletalMeshComponent`) `Visible?`)
  (`PrimitiveComponent.SetRenderCustomDepth` (`self.Bow`) `Visible?`)
  (`PrimitiveComponent.SetRenderCustomDepth` (`self.Arrow`) `Visible?`)
  (`PrimitiveComponent.SetRenderCustomDepth` (`self.LeftWeapon`) `Visible?`)
  (`PrimitiveComponent.SetRenderCustomDepth` (`self.Backpack`) `Visible?`)
  (`PrimitiveComponent.SetRenderCustomDepth` (`self.RightWeapon`) `Visible?`)
  (`PrimitiveComponent.SetRenderCustomDepth` (`self.Shield`) `Visible?`)
  (`PrimitiveComponent.SetRenderCustomDepth` (`self.ShoulderPad`) `Visible?`)
  (`PrimitiveComponent.SetRenderCustomDepth` (`self.Belt`) `Visible?`)
  (`PrimitiveComponent.SetRenderCustomDepth` (`self.HeadGears`) `Visible?`)
  (`PrimitiveComponent.SetRenderCustomDepth` (`self.Shoe`) `Visible?`)
  (`PrimitiveComponent.SetRenderCustomDepth` (`self.Glove`) `Visible?`)
  (`PrimitiveComponent.SetRenderCustomDepth` (`self.Hair`) `Visible?`)
  (`PrimitiveComponent.SetRenderCustomDepth` (`self.Face`) `Visible?`))

(fn `UpdateSkin`
  (`SkinnedMeshComponent.SetLeaderPoseComponent` (`self.Hair`) (`self.SkeletalMeshComponent`) false false)
  (`SkinnedMeshComponent.SetLeaderPoseComponent` (`self.Glove`) (`self.SkeletalMeshComponent`) false false)
  (`SkinnedMeshComponent.SetLeaderPoseComponent` (`self.Shoe`) (`self.SkeletalMeshComponent`) false false)
  (`SkinnedMeshComponent.SetLeaderPoseComponent` (`self.HeadGears`) (`self.SkeletalMeshComponent`) false false)
  (`SkinnedMeshComponent.SetLeaderPoseComponent` (`self.ShoulderPad`) (`self.SkeletalMeshComponent`) false false)
  (`SkinnedMeshComponent.SetLeaderPoseComponent` (`self.Belt`) (`self.SkeletalMeshComponent`) false false)
  (`SkinnedMeshComponent.SetLeaderPoseComponent` (`self.Face`) (`self.SkeletalMeshComponent`) false false))

(fn `UserConstructionScript`)