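; Manager actor that builds the tile grid and drives tile highlighting for character moves, switches and attacks.
; On BeginPlay it registers with BP_TopDownGameMode, then spawns BP_Tiles from DT_TileManager's dimensions and spacing, indexing each as row*10+column.
; Check functions match given indices against tile occupancy, activating empty tiles for moves and allied ones for switches, or returning an enemy's tile for attacks (-1 if none).
; Other functions reset tiles to neutral.
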(event `self.ReceiveBeginPlay`
  (bind (_returnvalue_x _returnvalue_y _returnvalue_z) (`KismetMathLibrary.BreakVector` (`self.K2_GetActorLocation`)))
  (bind (_ligne _colonne _espacement) (break `/Game/DataTable/Structure/Struct_TileManager` (`self.DTTileManager`)))
  (bind _asbp_top_down_game_mode (cast `/Game/TopDown/Blueprints/BP_TopDownGameMode` (`GameplayStatics.GetGameMode`)))
  (set `/Game/TopDown/Blueprints/BP_TopDownGameMode.TileManager` self _asbp_top_down_game_mode)
  (bind _returnvalue (`|GetDataTableRow` "/Game/DataTable/DT_TileManager.DT_TileManager" "TileManager")
    (:`then`
      (set `self.DTTileManager` _returnvalue)
      (`KismetSystemLibrary.DelayUntilNextTick`)
      (for _index (range _ligne)
        (for _index_2 (range _colonne)
          (bind _returnvalue_2 (`|SpawnActorFromClass` "/Game/Map/Tiles/BP_Tiles.BP_Tiles_C" (`KismetMathLibrary.MakeTransform` (`KismetMathLibrary.MakeVector` (+ (* _index _espacement) _returnvalue_x) (+ (* _index_2 _espacement) _returnvalue_y) _returnvalue_z)) "Undefined" "MultiplyWithRoot" null self (+ (* _index 10) _index_2) null))
          (`KismetArrayLibrary.Array_Add` (`self.AllTiles`) _returnvalue_2))))))

(fn `BlackOtherTiles`
  (for _array_element (`self.AllTiles`)
    (switch `/Game/DataTable/Enum/Enum_Tile` (`/Game/Map/Tiles/BP_Tiles.EtatTile` _array_element)
      (:`NewEnumerator0`
        _)
      (:`NewEnumerator1`
        _)
      (:`NewEnumerator4`
        _)
      (:`NewEnumerator3`
        _))
    (`/Game/Map/Tiles/BP_Tiles.ChangeEtat` _array_element "NewEnumerator0")))

(fn `CheckTileAttack`
  (params (TileAttaked :type "Array of Integer"))
  (returns (TileAttack :type Integer))
  (locals (`FindEnnemi?` :type Boolean) (EnnemieTouch :type "/Game/Personnage/Ennemie/BP_Ennemie Object Reference"))
  (for _array_element (`self.AllTiles`) :!label _label
    (for _array_element_2 TileAttaked
      (bind _reftile (`/Game/Map/Tiles/BP_Tiles.RefTile` _array_element))
      (if (== _array_element_2 _reftile)
        (bind (_hitactor _caseoccupee_) (`/Game/Map/Tiles/BP_Tiles.CheckChara` _array_element))
        (switch `/Game/DataTable/Enum/Enum_CheckTile` _caseoccupee_
          (:`NewEnumerator2`
            (set `local.FindEnnemi?` true)
            (`|ExecutionSequence`
              (:`then_0`
                (break))
              (:`then_1`
                (goto _label :!via `Break`))))))))
  (if (`local.FindEnnemi?`)
    (return _reftile)
    (else
      (return -1))))

(fn `CheckTileMove`
  (params (TileToCheckMove :type "Array of Integer") (TileToCheckSwitch :type "Array of Integer"))
  (locals (`CheckTileActive?` :type Boolean))
  (for _array_element (`self.AllTiles`)
    (set `local.CheckTileActive?` false)
    (for _array_element_2 TileToCheckMove
      (if (== _array_element_2 (`/Game/Map/Tiles/BP_Tiles.RefTile` _array_element))
        (bind (_hitactor _caseoccupee_) (`/Game/Map/Tiles/BP_Tiles.CheckChara` _array_element))
        (switch `/Game/DataTable/Enum/Enum_CheckTile` _caseoccupee_
          (:`NewEnumerator0`
            (set `local.CheckTileActive?` true)
            (`/Game/Map/Tiles/BP_Tiles.ChangeEtat` _array_element "NewEnumerator2")))))
    (for _array_element_3 TileToCheckSwitch
      (if (== _array_element_3 (`/Game/Map/Tiles/BP_Tiles.RefTile` _array_element))
        (bind (_hitactor_2 _caseoccupee__2) (`/Game/Map/Tiles/BP_Tiles.CheckChara` _array_element))
        (switch `/Game/DataTable/Enum/Enum_CheckTile` _caseoccupee__2
          (:`NewEnumerator1`
            (set `local.CheckTileActive?` true)
            (`/Game/Map/Tiles/BP_Tiles.ChangeEtat` _array_element "NewEnumerator5")))))))

(fn `CheckTileSwitch`
  (params (TileToCheck :type "Array of Integer"))
  (for _array_element (`self.AllTiles`)
    (for _array_element_2 TileToCheck
      (if (== _array_element_2 (`/Game/Map/Tiles/BP_Tiles.RefTile` _array_element))
        (bind (_hitactor _caseoccupee_) (`/Game/Map/Tiles/BP_Tiles.CheckChara` _array_element))
        (switch `/Game/DataTable/Enum/Enum_CheckTile` _caseoccupee_
          (:`NewEnumerator1`
            (`/Game/Map/Tiles/BP_Tiles.ChangeEtat` _array_element "NewEnumerator5")
            (break)))))))

(fn `DeactivateAllTiles`
  (for _array_element (`self.AllTiles`)
    (`/Game/Map/Tiles/BP_Tiles.ChangeEtat` _array_element "NewEnumerator0")))

(fn `UserConstructionScript`)