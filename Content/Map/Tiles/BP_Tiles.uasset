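; Grid tile for turn-based tactical combat that handles hovering and clicking to select allies, preview and execute moves, switches and attacks.
; Cursor events branch on combat phase and selection state held in RefManager, then drive BP_Personnage movement and attacks under action limits.
; Switches apply class effects: Guerrier and Combattant boosts, or a second tile pick for Archer teleports.
; Short upward traces detect occupants, while a dynamic overlay material shows each tile state.
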(event `self.ReceiveBeginPlay`
  (bind _asbp_top_down_game_mode (cast `/Game/TopDown/Blueprints/BP_TopDownGameMode` (`GameplayStatics.GetGameMode`)))
  (set `self.GM` _asbp_top_down_game_mode))

(event `self.StaticMesh.OnBeginCursorOver`
  (params (TouchedComponent :type "PrimitiveComponent Object Reference"))
  (bind _asbp_personnage (cast `/Game/Personnage/BP_Personnage` (`/Game/Map/Tiles/BP_TileManager.PersoActif` (`self.RefManager`)) :!pure true))
  ;[0.05 0.05 0.05] Over
  (`self.WhichPhase?`
    (:`DepJoueur`
      (if (< (`/Game/Map/Tiles/BP_TileManager.NumberActionRedp` (`self.RefManager`)) 1)
        (`self.CheckChangeTile`)
        (`self.CheckClicked`
          (:`Yes`
            (switch `/Game/DataTable/Enum/Enum_Tile` (`self.EtatTile`)
              (:`NewEnumerator6`
                (`self.ChangeEtat` "NewEnumerator2"))
              (:`NewEnumerator7`
                (`self.ChangeEtat` "NewEnumerator5"))))
          (:`No`
            (`self.AffichePerso`)
            (`/Game/Map/Tiles/BP_TileManager.DeactivateAllTiles` (`self.RefManager`))
            (bind (_hitactor _caseoccupee_) (`self.CheckChara`))
            (switch `/Game/DataTable/Enum/Enum_CheckTile` _caseoccupee_
              (:`NewEnumerator1`
                (bind _asbp_personnage_2 (cast `/Game/Personnage/BP_Personnage` _hitactor))
                (`/Game/Personnage/BP_Personnage.DeplacementClassic` _asbp_personnage_2 (`self.RefTile`))))))))
    (:`ActionJoueur`
      (`self.CheckChangeTile`)
      (`self.CheckClicked`
        (:`Yes`
          (if (not (`/Game/Map/Tiles/BP_TileManager.TpArcher?` (`self.RefManager`)))
            (switch `/Game/DataTable/Enum/Enum_Tile` (`self.EtatTile`)
              (:`NewEnumerator6`
                (`self.ChangeEtat` "NewEnumerator2"))
              (:`NewEnumerator7`
                (`self.ChangeEtat` "NewEnumerator5")))
            (`/Engine/EditorBlueprintResources/StandardMacros.IsValid` _asbp_personnage
              (:`Is Valid`
                (`/Game/Personnage/BP_ParentPerso.AtkPuissante` _asbp_personnage (`self.RefTile`) false)))
            (else
              (switch `/Game/DataTable/Enum/Enum_Tile` (`self.EtatTile`)
                (:`NewEnumerator6`
                  (`self.ChangeEtat` "NewEnumerator2"))))))
        (:`No`
          (`self.AffichePerso`)
          (`/Game/Map/Tiles/BP_TileManager.DeactivateAllTiles` (`self.RefManager`))
          (bind (_hitactor_2 _caseoccupee__2) (`self.CheckChara`))
          (switch `/Game/DataTable/Enum/Enum_CheckTile` _caseoccupee__2
            (:`NewEnumerator1`
              (bind _asbp_personnage_3 (cast `/Game/Personnage/BP_Personnage` _hitactor_2))
              (`/Game/Personnage/BP_Personnage.DeplacementAction` _asbp_personnage_3 (`self.RefTile`)))))))))

(event `self.StaticMesh.OnClicked`
  (params (TouchedComponent :type "PrimitiveComponent Object Reference") (ButtonPressed :type "Key Structure"))
  (bind _refmanager (`self.RefManager`))
  (bind _refmanager_2 (`self.RefManager`))
  (bind _refmanager_3 (`self.RefManager`))
  (bind _refmanager_4 (`self.RefManager`))
  (bind _refmanager_5 (`self.RefManager`))
  (bind _refmanager_6 (`self.RefManager`))
  (bind _refmanager_7 (`self.RefManager`))
  (bind _asbp_personnage (cast `/Game/Personnage/BP_Personnage` (`/Game/Map/Tiles/BP_TileManager.PersoActif` (`self.RefManager`)) :!pure true))
  (bind _asbp_personnage_2 (cast `/Game/Personnage/BP_Personnage` (`/Game/Map/Tiles/BP_TileManager.PersoActif` (`self.RefManager`)) :!pure true))
  (bind _asbp_personnage_3 (cast `/Game/Personnage/BP_Personnage` (`/Game/Map/Tiles/BP_TileManager.PersoActif` (`self.RefManager`)) :!pure true))
  (bind _asbp_personnage_4 (cast `/Game/Personnage/BP_Personnage` (`/Game/Map/Tiles/BP_TileManager.PersoSwitch` (`self.RefManager`)) :!pure true))
  (bind _asbp_personnage_5 (cast `/Game/Personnage/BP_Personnage` (`/Game/Map/Tiles/BP_TileManager.PersoSwitch` (`self.RefManager`)) :!pure true))
  (bind _asbp_personnage_6 (cast `/Game/Personnage/BP_Personnage` (`/Game/Map/Tiles/BP_TileManager.PersoActif` (`self.RefManager`)) :!pure true))
  (bind _asbp_weapon_parent (cast `/Game/Personnage/Weapon/BP_WeaponParent` (`ChildActorComponent.ChildActor` (`/Game/Personnage/BP_Personnage.WeaponR` _asbp_personnage)) :!pure true))
  ;[0.05 0.05 0.05] Clicked
  (`self.WhichPhase?`
    (:`DepJoueur`
      (if (< (`/Game/Map/Tiles/BP_TileManager.NumberActionRedp` (`self.RefManager`)) 1)
        (`self.CheckClicked`
          (:`Yes`
            (switch `/Game/DataTable/Enum/Enum_Tile` (`self.EtatTile`)
              (:`NewEnumerator2`
                (`/Game/Personnage/BP_ParentPerso.MoveChara` _asbp_personnage_6 (`self.K2_GetActorLocation`))
                (`/Game/Personnage/BP_Personnage.AlreadyPlayed?` _asbp_personnage_6 true)
                (set `self.ChangeTile?` false)
                (set `/Game/Map/Tiles/BP_TileManager.Clicked?` false _refmanager_3)
                (`/Game/Map/Tiles/BP_TileManager.DeactivateAllTiles` _refmanager_3)
                (`/Game/Map/Tiles/BP_TileManager.Change Number Action Redep` (`self.RefManager`) false))))
          (:`No`
            (bind (_hitactor _caseoccupee_) (`self.CheckChara`))
            (switch `/Game/DataTable/Enum/Enum_CheckTile` _caseoccupee_
              (:`NewEnumerator1`
                (set `/Game/Map/Tiles/BP_TileManager.PersoActif` _hitactor _refmanager_7)
                (bind _asbp_personnage_7 (cast `/Game/Personnage/BP_Personnage` _hitactor))
                (if (not (`/Game/Personnage/BP_Personnage.AlreadyPlay?` _asbp_personnage_7))
                  (set `/Game/Map/Tiles/BP_TileManager.Clicked?` true _refmanager_7))))))))
    (:`ActionJoueur`
      (if (`self.ChangeTile?`)
        (if (< (`/Game/Map/Tiles/BP_TileManager.NumberActionAtk` (`self.RefManager`)) 2)
          (`self.CheckClicked`
            (:`Yes`
              (switch `/Game/DataTable/Enum/Enum_Tile` (`self.EtatTile`)
                (:`NewEnumerator2`
                  (if (not (`/Game/Map/Tiles/BP_TileManager.TpArcher?` (`self.RefManager`)))
                    (bind _asbp_personnage_8 (cast `/Game/Personnage/BP_Personnage` (`/Game/Map/Tiles/BP_TileManager.PersoActif` (`self.RefManager`))))
                    (`/Game/Personnage/BP_Personnage.AlreadyPlayed?` _asbp_personnage_8 true)
                    (`/Game/Personnage/BP_Personnage.MoveChara` _asbp_personnage_8 (`self.K2_GetActorLocation`))
                    (`/Game/Personnage/BP_ParentPerso.AtkPuissante` _asbp_personnage_8 (`self.RefTile`) true)
                    (set `/Game/Map/Tiles/BP_TileManager.Clicked?` false _refmanager_2)
                    (`/Game/Map/Tiles/BP_TileManager.DeactivateAllTiles` _refmanager_2)
                    (set `self.ChangeTile?` false)
                    (`/Game/Map/Tiles/BP_TileManager.Change Number Action Atk` (`self.RefManager`) false)
                    (else
                      (set `self.SwitchLocation` (`self.K2_GetActorLocation` _asbp_personnage_4))
                      (`/Game/Personnage/BP_Personnage.MoveChara` _asbp_personnage_4 (`self.K2_GetActorLocation`))
                      (`|ExecutionSequence`
                        (:`then_0`
                          (`/Game/Personnage/BP_Personnage.MoveChara` _asbp_personnage_2 (`self.SwitchLocation`))
                          (`/Game/Personnage/BP_Personnage.AlreadyPlayed?` _asbp_personnage_2 true)
                          (bind _reftile (`/Game/Personnage/BP_Personnage.RecupTile` _asbp_personnage_2))
                          (`/Game/Personnage/BP_ParentPerso.AtkPuissante` _asbp_personnage_2 _reftile true)
                          (set `self.ChangeTile?` false)
                          (set `/Game/Map/Tiles/BP_TileManager.Clicked?` false _refmanager_4)
                          (set `/Game/Map/Tiles/BP_TileManager.TpArcher?` false _refmanager_4)
                          (`/Game/Map/Tiles/BP_TileManager.DeactivateAllTiles` _refmanager_4)
                          (`/Game/Map/Tiles/BP_TileManager.Change Number Action Atk` _refmanager_4 false))
                        (:`then_1`
                          (`KismetSystemLibrary.Delay` 0.7)
                          (`/Game/Personnage/BP_ParentPerso.AtkRapide` _asbp_personnage_4 (`self.RefTile`) true))))))
                (:`NewEnumerator5`
                  (bind _hitactor_2 (`self.CheckChara`))
                  (bind _asbp_personnage_9 (cast `/Game/Personnage/BP_Personnage` _hitactor_2))
                  (set `/Game/Map/Tiles/BP_TileManager.PersoSwitch` _asbp_personnage_9 (`self.RefManager`))
                  (set `self.SwitchLocation` (`self.K2_GetActorLocation` _asbp_personnage_9))
                  (switch `/Game/DataTable/Enum/Enum_Classes` (`/Game/Personnage/BP_ParentPerso.Classes` _asbp_personnage)
                    (:`NewEnumerator0`
                      (bind _hitactor_3 (`self.CheckChara`))
                      (bind _asbp_personnage_10 (cast `/Game/Personnage/BP_Personnage` _hitactor_3))
                      (`/Game/Personnage/Weapon/BP_WeaponParent.BoostPerso` _asbp_weapon_parent (`self.RefTile`) false true -2)
                      (`/Game/UI/WB_HPBar.PlayAnimDamage` (`/Game/Personnage/BP_ParentPerso.WB HPBar` _asbp_personnage_10) -2)
                      (`/Game/Personnage/BP_Personnage.MoveChara` _asbp_personnage_9 (`self.K2_GetActorLocation` _asbp_personnage_3) :!label _label)
                      (`/Game/Personnage/BP_Personnage.MoveChara` _asbp_personnage_3 (`self.SwitchLocation`))
                      (`/Game/Personnage/BP_Personnage.AlreadyPlayed?` _asbp_personnage_3 true)
                      (`/Game/Personnage/BP_ParentPerso.AtkPuissante` _asbp_personnage_3 (`self.RefTile`) true)
                      (`|ExecutionSequence`
                        (:`then_0`
                          (set `self.ChangeTile?` false)
                          (set `/Game/Map/Tiles/BP_TileManager.Clicked?` false _refmanager_6)
                          (`/Game/Map/Tiles/BP_TileManager.DeactivateAllTiles` _refmanager_6)
                          (`/Game/Map/Tiles/BP_TileManager.Change Number Action Atk` (`self.RefManager`) false))
                        (:`then_1`
                          (`KismetSystemLibrary.Delay` 0.9)
                          (bind _reftile_2 (`/Game/Personnage/BP_ParentPerso.RecupTile` _asbp_personnage_5))
                          (`/Game/Personnage/BP_ParentPerso.AtkRapide` _asbp_personnage_5 _reftile_2 true))))
                    (:`NewEnumerator3`
                      (bind _hitactor_4 (`self.CheckChara`))
                      (bind _asbp_personnage_11 (cast `/Game/Personnage/BP_Personnage` _hitactor_4))
                      (`/Game/Personnage/Weapon/BP_WeaponParent.BoostPerso` _asbp_weapon_parent (`self.RefTile`) false true -2)
                      (`/Game/UI/WB_HPBar.PlayAnimDamage` (`/Game/Personnage/BP_ParentPerso.WB HPBar` _asbp_personnage_11) -2)
                      (bind _reftile_3 (`/Game/Personnage/BP_Personnage.RecupTile` _asbp_personnage))
                      (`/Game/Personnage/Weapon/BP_WeaponParent.BoostPerso` _asbp_weapon_parent _reftile_3 false true -2)
                      (`/Game/UI/WB_HPBar.PlayAnimDamage` (`/Game/Personnage/BP_ParentPerso.WB HPBar` _asbp_personnage) -2)
                      (goto _label))
                    (:`NewEnumerator1`
                      (bind _reftile_4 (`/Game/Personnage/BP_Personnage.RecupTile` _asbp_personnage))
                      (`/Game/Personnage/Weapon/BP_WeaponParent.BoostPerso` _asbp_weapon_parent _reftile_4 true false 2)
                      (goto _label))
                    (:`NewEnumerator4`
                      (bind _reftile_5 (`/Game/Personnage/BP_Personnage.RecupTile` _asbp_personnage))
                      (`/Game/Personnage/Weapon/BP_WeaponParent.BoostPerso` _asbp_weapon_parent _reftile_5 true false 3)
                      (goto _label))
                    (:`NewEnumerator2`
                      (set `/Game/Map/Tiles/BP_TileManager.TpArcher?` true _refmanager :!label _label_2)
                      (`/Game/Map/Tiles/BP_TileManager.DeactivateAllTiles` _refmanager)
                      (`/Game/Map/Tiles/BP_TileManager.FindAllyTilesLibre` _refmanager))
                    (:`NewEnumerator5`
                      (goto _label_2))))))
            (:`No`
              (bind (_hitactor_5 _caseoccupee__2) (`self.CheckChara`))
              (switch `/Game/DataTable/Enum/Enum_CheckTile` _caseoccupee__2
                (:`NewEnumerator1`
                  (set `/Game/Map/Tiles/BP_TileManager.PersoActif` _hitactor_5 _refmanager_5)
                  (bind _asbp_personnage_12 (cast `/Game/Personnage/BP_Personnage` _hitactor_5))
                  (if (not (`/Game/Personnage/BP_Personnage.AlreadyPlay?` _asbp_personnage_12))
                    (set `/Game/Map/Tiles/BP_TileManager.Clicked?` true _refmanager_5)))))))))))

(event `self.StaticMesh.OnEndCursorOver`
  (params (TouchedComponent :type "PrimitiveComponent Object Reference"))
  ;[0.05 0.05 0.05] End Cursor Over
  (`self.CheckClicked`
    (:`Yes`
      (switch `/Game/DataTable/Enum/Enum_Tile` (`self.EtatTile`)
        (:`NewEnumerator2`
          _)
        (:`NewEnumerator5`
          _))
      (for _array_element (`/Game/Map/Tiles/BP_TileManager.AllTiles` (`self.RefManager`))
        (switch `/Game/DataTable/Enum/Enum_Tile` (`/Game/Map/Tiles/BP_Tiles.EtatTile` _array_element)
          (:`NewEnumerator2`
            (`self.ChangeEtat` "NewEnumerator6"))
          (:`NewEnumerator5`
            (`self.ChangeEtat` _array_element "NewEnumerator7"))
          (:`NewEnumerator3`
            (`self.ChangeEtat` _array_element "NewEnumerator0")
            (bind _hitactor (`self.CheckChara` _array_element))
            (bind _asbp_ennemie (cast `/Game/Personnage/Ennemie/BP_Ennemie` _hitactor))
            (`/Game/UI/WB_HPBar.UpdateBoxDamage` (`/Game/Personnage/Ennemie/BP_Ennemie.WB HPBar` _asbp_ennemie) "Collapsed" 0)))))
    (:`No`
      (set `/Game/UI/WB_MainCombat.EslatePerso` "Collapsed" (`/Game/TopDown/Blueprints/BP_TopDownGameMode.WBMainCombat` (`/Game/Map/Tiles/BP_TileManager.GM` (`self.RefManager`))))
      (for _array_element_2 (`/Game/Map/Tiles/BP_TileManager.AllTiles` (`self.RefManager`))
        (`self.ChangeEtat` _array_element_2 "NewEnumerator0")))))

(event `self.StaticMesh.OnReleased`
  (params (TouchedComponent :type "PrimitiveComponent Object Reference") (ButtonReleased :type "Key Structure"))
  ;[0.05 0.05 0.05] OnReleased
  (`self.CheckClicked`))

(fn `AffichePerso`
  (bind _wbmaincombat (`/Game/TopDown/Blueprints/BP_TopDownGameMode.WBMainCombat` (`/Game/Map/Tiles/BP_TileManager.GM` (`self.RefManager`))))
  (bind (_hitactor _caseoccupee_) (`self.CheckChara`))
  (switch `/Game/DataTable/Enum/Enum_CheckTile` _caseoccupee_
    (:`NewEnumerator1`
      _)
    (:`NewEnumerator2`
      _))
  (set `/Game/UI/WB_MainCombat.EslatePerso` "Visible" _wbmaincombat)
  (`/Game/UI/WB_MainCombat.UpdatePerso` _wbmaincombat (cast `/Game/Personnage/BP_ParentPerso` _hitactor :!pure true)))

(fn `ChangeEtat`
  (params (Material :type "/Game/DataTable/Enum/Enum_Tile Enum" :default "NewEnumerator0"))
  (locals (LMove :type "LinearColor Structure" :default (struct :`G` 0.084376 :`B` 0.672443 :`A` 1.0)) (LSwitch :type "LinearColor Structure" :default (struct :`G` 0.629174 :`B` 0.672443 :`A` 1.0)))
  (bind _lmove (`local.LMove`))
  (bind _lswitch (`local.LSwitch`))
  (set `self.EtatTile` Material)
  (switch `/Game/DataTable/Enum/Enum_Tile` Material
    (:`NewEnumerator0`
      (`self.EmissiveTiles` (struct)))
    (:`NewEnumerator1`
      (`self.EmissiveTiles` (struct :`R` 0.953125 :`G` 0.953125 :`B` 0.953125 :`A` 0.942) 0.5 0.5))
    (:`NewEnumerator6`
      (`self.EmissiveTiles` _lmove 0.25 0.5))
    (:`NewEnumerator2`
      (`self.EmissiveTiles` _lmove 1.0 0.5))
    (:`NewEnumerator7`
      (`self.EmissiveTiles` _lswitch 0.35 0.5))
    (:`NewEnumerator5`
      (`self.EmissiveTiles` _lswitch 1.0 0.75))
    (:`NewEnumerator4`
      (`self.EmissiveTiles` (struct :`R` 1.0 :`G` 1.0 :`B` 1.0 :`A` 0.25)))
    (:`NewEnumerator3`
      (`self.EmissiveTiles` (struct :`R` 0.734375 :`B` 0.02062 :`A` 1.0) 2.0 0.75)))
  (`MeshComponent.SetOverlayMaterial` (`self.StaticMesh`) (`self.MITilesRef`)))

(fn `CheckChangeTile`
  (for _array_element (`/Game/Map/Tiles/BP_TileManager.AllTiles` (`self.RefManager`))
    (set `/Game/Map/Tiles/BP_Tiles.ChangeTile?` true _array_element)))

(fn `CheckChara`
  (returns (HitActor :type "Actor Object Reference") (`CaseOccupee?` :type "/Game/DataTable/Enum/Enum_CheckTile Enum"))
  (bind _returnvalue (`self.K2_GetActorLocation`))
  (bind _returnvalue_2 (`self.K2_GetActorLocation`))
  (bind (_outhit _returnvalue_3) (`KismetSystemLibrary.LineTraceSingleForObjects` _returnvalue_2 (+ _returnvalue_2 (0.0 0.0 75.0)) (`|MakeArray` "ObjectTypeQuery7" :!type "EObjectTypeQuery Enum")))
  (if _returnvalue_3
    (return (`.HitActor` (`GameplayStatics.BreakHitResult` _outhit)) "NewEnumerator1")
    (else
      (bind (_outhit_2 _returnvalue_4) (`KismetSystemLibrary.LineTraceSingleForObjects` _returnvalue (+ _returnvalue (0.0 0.0 75.0)) (`|MakeArray` "ObjectTypeQuery8" :!type "EObjectTypeQuery Enum")))
      (if _returnvalue_4
        (return (`.HitActor` (`GameplayStatics.BreakHitResult` _outhit_2)) "NewEnumerator2")
        (else
          (return null "NewEnumerator0"))))))

(fn `EmissiveTiles`
  (params (Value :type "LinearColor Structure") (Emissive :type "Float (single-precision)") (Opacity :type "Float (single-precision)"))
  (`MaterialInstanceDynamic.SetVectorParameterValue` (`self.MITilesRef`) "EmissiveColor" Value)
  (`MaterialInstanceDynamic.SetScalarParameterValue` (`self.MITilesRef`) "Emissive" Emissive)
  (`MaterialInstanceDynamic.SetScalarParameterValue` (`self.MITilesRef`) "Opacity" Opacity)
  (return))

(fn `UserConstructionScript`
  (bind _returnvalue (`KismetMaterialLibrary.CreateDynamicMaterialInstance` (`self.MITiles`)))
  (set `self.MITilesRef` _returnvalue))