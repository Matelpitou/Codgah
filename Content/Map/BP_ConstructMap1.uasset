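; Map actor that builds a grid of hex tile meshes in its Construction Script.
; The TileMap row of DT_TileManager supplies row and column counts and spacing, and a first pass appends SM_Tile_Hex_Flat_01 per tile.
; A second pass spawns mesh components offset from the actor location, applying mesh and rotation by index.
; The row-index branch places tiles identically on both sides, and the Rotation fill is unconnected.
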(event `self.ReceiveBeginPlay`)

(fn `UserConstructionScript`
  (bind (_returnvalue_x _returnvalue_y _returnvalue_z) (`KismetMathLibrary.BreakVector` (`self.K2_GetActorLocation`)))
  (bind (_returnvalue_x_2 _returnvalue_y_2 _returnvalue_z_2) (`KismetMathLibrary.BreakVector` (`self.K2_GetActorLocation`)))
  (`|ExecutionSequence`
    (:`then_0`
      (bind _returnvalue (`|GetDataTableRow` "/Game/DataTable/DT_TileManager.DT_TileManager" "TileMap")
        (:`then`
          (bind (_ligne _colonne) (break `/Game/DataTable/Structure/Struct_TileManager` _returnvalue))
          (for _ (range (+ (* _ligne _colonne) 1))
            (`KismetArrayLibrary.Array_Add` (`self.StaticMesh`) "/Game/Package/PolygonMini_Fantasy/Meshes/Tiles/SM_Tile_Hex_Flat_01.SM_Tile_Hex_Flat_01")))))
    (:`then_1`
      (bind _returnvalue_2 (`|GetDataTableRow` "/Game/DataTable/DT_TileManager.DT_TileManager" "TileMap")
        (:`then`
          (bind (_ligne_2 _colonne_2 _espacementligne _espacementcolonne) (break `/Game/DataTable/Structure/Struct_TileManager` _returnvalue_2))
          (for _index (range (+ _ligne_2 1))
            (if (or (== _index 1) (== _index 1) (== _index 1) (== _index 1) (== _index 1))
              (for _index_2 (range (+ _colonne_2 1))
                (bind _returnvalue_3 (`AddComponent|NODE_AddStaticMeshComponent-1` :`bManualAttachment` true :`RelativeTransform` (`KismetMathLibrary.MakeTransform` (`KismetMathLibrary.MakeVector` (+ (* _index _espacementligne) _returnvalue_x) (+ (* _index_2 _espacementcolonne) _returnvalue_y) _returnvalue_z))))
                (bind _returnvalue_4 (`KismetArrayLibrary.Array_Add` (`self.AllSM`) _returnvalue_3))
                (bind _output (`|GetArrayItem` (`self.AllSM`) _returnvalue_4))
                (`StaticMeshComponent.SetStaticMesh` _output (`|GetArrayItem` (`self.StaticMesh`) _returnvalue_4))
                (`SceneComponent.K2_SetWorldRotation` _output (`|GetArrayItem` (`self.Rotation`) _returnvalue_4) false false))
              (else
                (for _index_3 (range (+ _colonne_2 1))
                  (bind _returnvalue_5 (`AddComponent|NODE_AddStaticMeshComponent-0` :`bManualAttachment` true :`RelativeTransform` (`KismetMathLibrary.MakeTransform` (`KismetMathLibrary.MakeVector` (+ (* _index _espacementligne) _returnvalue_x_2) (+ (* _index_3 _espacementcolonne) _returnvalue_y_2) _returnvalue_z_2))))
                  (bind _returnvalue_6 (`KismetArrayLibrary.Array_Add` (`self.AllSM`) _returnvalue_5))
                  (bind _output_2 (`|GetArrayItem` (`self.AllSM`) _returnvalue_6))
                  (`StaticMeshComponent.SetStaticMesh` _output_2 (`|GetArrayItem` (`self.StaticMesh`) _returnvalue_6))
                  (`SceneComponent.K2_SetWorldRotation` _output_2 (`|GetArrayItem` (`self.Rotation`) _returnvalue_6) false false))))))))))