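; BP_ConstructMap builds a grid of static mesh tiles for the map in its construction script.
; The TileCbt row of DT_TileManager supplies row and column counts and spacing, with positions offset from the actor's location.
; Each manually attached component is stored in AllSM, and its index picks the mesh and world rotation from the parallel StaticMesh and Rotation arrays.
; Unconnected nodes for filling those arrays never run, and BeginPlay is empty.
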(event `self.ReceiveBeginPlay`)

(fn `UserConstructionScript`
  (bind (_returnvalue_x _returnvalue_y _returnvalue_z) (`KismetMathLibrary.BreakVector` (`self.K2_GetActorLocation`)))
  (`|ExecutionSequence`
    (:`then_1`
      (bind _returnvalue (`|GetDataTableRow` "/Game/DataTable/DT_TileManager.DT_TileManager" "TileCbt")
        (:`then`
          (bind (_ligne _colonne _espacementligne _espacementcolonne) (break `/Game/DataTable/Structure/Struct_TileManager` _returnvalue))
          (for _index (range (+ _ligne 1))
            (for _index_2 (range (+ _colonne 1))
              (bind _returnvalue_2 (`AddComponent|NODE_AddStaticMeshComponent-0` :`bManualAttachment` true :`RelativeTransform` (`KismetMathLibrary.MakeTransform` (`KismetMathLibrary.MakeVector` (+ (* _index _espacementligne) _returnvalue_x) (+ (* _index_2 _espacementcolonne) _returnvalue_y) _returnvalue_z))))
              (bind _returnvalue_3 (`KismetArrayLibrary.Array_Add` (`self.AllSM`) _returnvalue_2))
              (bind _output (`|GetArrayItem` (`self.AllSM`) _returnvalue_3))
              (`StaticMeshComponent.SetStaticMesh` _output (`|GetArrayItem` (`self.StaticMesh`) _returnvalue_3))
              (`SceneComponent.K2_SetWorldRotation` _output (`|GetArrayItem` (`self.Rotation`) _returnvalue_3) false false))))))))