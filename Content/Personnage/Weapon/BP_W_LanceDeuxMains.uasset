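; Two-handed lance weapon for tile-based combat, extending a parent weapon with its own heavy and quick attacks.
; Heavy attack runs the classic hit and move-to-attack, then strikes enemies one and two tiles past the target for half damage.
; The Damage flag switches HitLance between applying damage and previewing it through tile state and HP bar.
; Quick attack adds a level-scaled enrage boost on the tile after the wielder's.
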(event `self.AttackPuissante`
  (params (RefTile :type Integer) (`Damage?` :type Boolean) (AtkRapide :type Integer) (AtkPuissante :type Integer) (Rage :type Integer) (EnumWeapon :type "/Game/DataTable/Enum/Enum_Armes Enum" :default "NewEnumerator0"))
  ;[0.05 0.05 0.05] Atk Puissante
  (`self.SetAttack` AtkRapide AtkPuissante Rage)
  (bind _tilecible (`self.AttackClassique` RefTile))
  (bind (_tileennemi _findenemy_) (`self.HitClassique` _tilecible `Damage?`))
  (`KismetSystemLibrary.DelayUntilNextTick`)
  (`self.MoveToAtkPlayer` _findenemy_ `Damage?` RefTile _tileennemi)
  (bind _tilecible_2 (`self.AttackBefore1` _tileennemi))
  (`self.Hit Lance` _tilecible_2 `Damage?`)
  (bind _tilecible_3 (`self.AttackBefore2` _tileennemi))
  (`self.Hit Lance` _tilecible_3 `Damage?`))

(event `self.AttackRapide`
  (params (RefTile :type Integer) (`Damage?` :type Boolean) (AtkRapide :type Integer) (AtkPuissante :type Integer) (Rage :type Integer) (EnumWeapon :type "/Game/DataTable/Enum/Enum_Armes Enum" :default "NewEnumerator0"))
  (bind _returnvalue (+ RefTile 1))
  ;[0.05 0.05 0.05] Atk Rapide
  (`parent.AttackRapide` RefTile `Damage?` AtkRapide AtkPuissante Rage EnumWeapon)
  (switch `/Game/DataTable/Enum/Enum_Armes` EnumWeapon
    (:`NewEnumerator3`
      (`self.BoostPerso` _returnvalue true false 1))
    (:`NewEnumerator12`
      (`self.BoostPerso` _returnvalue true false 2))))

(fn `AttackBefore1`
  (params (RefTile :type Integer))
  (returns (TileCible :type "Array of Integer"))
  (locals (LRefTile :type Integer) (TileAttack :type "Array of Integer"))
  (set `local.LRefTile` RefTile)
  (`KismetArrayLibrary.Array_Add` (`local.TileAttack`) (+ (`local.LRefTile`) 1))
  (return (`local.TileAttack`)))

(fn `AttackBefore2`
  (params (RefTile :type Integer))
  (returns (TileCible :type "Array of Integer"))
  (locals (TileAttack :type "Array of Integer") (LRefTile :type Integer))
  (set `local.LRefTile` RefTile)
  (`KismetArrayLibrary.Array_Add` (`local.TileAttack`) (+ (`local.LRefTile`) 2))
  (return (`local.TileAttack`)))

(fn `Hit Lance`
  (params (TileAttaked :type "Array of Integer (by ref)") (`Damage?` :type Boolean) (`Rapide?` :type Boolean))
  (returns (TileEnnemi :type Integer))
  (locals (LReduce :type Boolean) (LRefTile :type Integer))
  (set `local.LReduce` false)
  (bind _tileattack (`/Game/Map/Tiles/BP_TileManager.CheckTileAttack` (`self.TileManager`) TileAttaked))
  (for _array_element (`/Game/Map/Tiles/BP_TileManager.AllTiles` (`self.TileManager`))
    (bind _reftile (`/Game/Map/Tiles/BP_Tiles.RefTile` _array_element))
    (if (== _reftile _tileattack)
      (set `local.LRefTile` _reftile)
      (if `Damage?`
        (bind (_hitactor _caseoccupee_) (`/Game/Map/Tiles/BP_Tiles.CheckChara` _array_element))
        (switch `/Game/DataTable/Enum/Enum_CheckTile` _caseoccupee_
          (:`NewEnumerator0`
            _)
          (:`NewEnumerator1`
            _)
          (:`NewEnumerator2`
            (bind _damage (`self.Calcul Damage` `Rapide?`))
            (bind _asbp_ennemie (cast `/Game/Personnage/Ennemie/BP_Ennemie` _hitactor :!pure true))
            (bind _divide (`self.DivideBy2` _damage))
            (`/Game/Personnage/Ennemie/BP_Ennemie.Takehit` _asbp_ennemie _divide false 0 false 0 false false false)
            (`/Game/UI/WB_HPBar.PlayAnimDamage` (`/Game/Personnage/Ennemie/BP_Ennemie.WB HPBar` _asbp_ennemie) _divide)
            (return (`local.LRefTile`))))
        (return -110)
        (else
          (`/Game/Map/Tiles/BP_Tiles.ChangeEtat` _array_element "NewEnumerator3")
          (bind _hitactor_2 (`/Game/Map/Tiles/BP_Tiles.CheckChara` _array_element))
          (bind _damage_2 (`self.Calcul Damage` `Rapide?`))
          (`/Game/UI/WB_HPBar.UpdateBoxDamage` (`/Game/Personnage/Ennemie/BP_Ennemie.WB HPBar` (cast `/Game/Personnage/Ennemie/BP_Ennemie` _hitactor_2 :!pure true)) "Visible" (`self.DivideBy2` _damage_2))
          (return (`local.LRefTile`)))))))

(fn `UserConstructionScript`
  (`parent.UserConstructionScript`))