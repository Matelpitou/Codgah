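; Crossbow (Arbalete) weapon Blueprint for tile-based combat, overriding the quick and heavy attacks of its parent weapon.
; Heavy attack enables armor break scaled by weapon level, then chains ally check, classic tile targeting, hit detection and move-to-attack.
; When its Damage flag is set, it also raises AlreadyAtk, which makes the next quick attack only clear that flag instead of running the parent logic.
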(event `self.AttackPuissante`
  (params (RefTile :type Integer) (`Damage?` :type Boolean) (AtkRapide :type Integer) (AtkPuissante :type Integer) (Rage :type Integer) (EnumWeapon :type "/Game/DataTable/Enum/Enum_Armes Enum" :default "NewEnumerator0"))
  ;[0.05 0.05 0.05] Atk Puissante
  (`|ExecutionSequence`
    (:`then_0`
      (switch `/Game/DataTable/Enum/Enum_Armes` EnumWeapon
        (:`NewEnumerator8`
          (set `self.Brise Armure?` true)
          (set `self.Armure` 3))
        (:`NewEnumerator17`
          (set `self.Brise Armure?` true)
          (set `self.Armure` 5))))
    (:`then_1`
      (`self.SetAttack` AtkRapide AtkPuissante Rage)
      (bind _ally_ (`self.CheckAlly?`))
      (bind _tilecible (`self.AtkClassique` RefTile _ally_))
      (bind (_tileennemi _findenemy_) (`self.HitClassique` _tilecible `Damage?` false _ally_))
      (`self.MoveToAtkPlayer` _findenemy_ `Damage?` RefTile _tileennemi)
      (if `Damage?`
        (set `self.AlreadyAtk?` true)))))

(event `self.AttackRapide`
  (params (RefTile :type Integer) (`Damage?` :type Boolean) (AtkRapide :type Integer) (AtkPuissante :type Integer) (Rage :type Integer) (EnumWeapon :type "/Game/DataTable/Enum/Enum_Armes Enum" :default "NewEnumerator0"))
  ;[0.05 0.05 0.05] Atk Rapide
  (if (`self.AlreadyAtk?`)
    (set `self.AlreadyAtk?` false)
    (else
      (`parent.AttackRapide` RefTile `Damage?` AtkRapide AtkPuissante Rage EnumWeapon))))

(fn `UserConstructionScript`
  (`parent.UserConstructionScript`))