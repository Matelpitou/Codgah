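; Base weapon for player characters in tile-based combat, providing quick and powerful attacks.
; Each attack feeds five tile offsets ahead to the TileManager, then either previews damage on the enemy's health bar or applies it with status effects and moves the owning character to strike.
; Damage is the chosen attack value plus Rage.
; BoostPerso boosts an ally's Rage or reuses TakeDamage, where negative values augment.
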(event `self.ReceiveBeginPlay`
  (`KismetSystemLibrary.DelayUntilNextTick`)
  (bind _asbp_top_down_game_mode (cast `/Game/TopDown/Blueprints/BP_TopDownGameMode` (`GameplayStatics.GetGameMode`)))
  (set `self.TileManager` (`/Game/TopDown/Blueprints/BP_TopDownGameMode.TileManager` _asbp_top_down_game_mode)))

(event `AttackPuissante`
  (params (RefTile :type Integer) (`Damage?` :type Boolean) (AtkRapide :type Integer) (AtkPuissante :type Integer) (Rage :type Integer) (EnumWeapon :type "/Game/DataTable/Enum/Enum_Armes Enum" :default "NewEnumerator0"))
  (`self.SetAttack` AtkRapide AtkPuissante Rage)
  (bind _tilecible (`self.AttackClassique` RefTile))
  (bind (_tileennemi _findenemy_) (`self.HitClassique` _tilecible `Damage?`))
  (`self.MoveToAtkPlayer` _findenemy_ `Damage?` RefTile _tileennemi))

(event `AttackRapide`
  (params (RefTile :type Integer) (`Damage?` :type Boolean) (AtkRapide :type Integer) (AtkPuissante :type Integer) (Rage :type Integer) (EnumWeapon :type "/Game/DataTable/Enum/Enum_Armes Enum" :default "NewEnumerator0"))
  (`self.SetAttack` AtkRapide AtkPuissante Rage)
  (bind _tilecible (`self.AttackClassique` RefTile))
  (bind (_tileennemi _findenemy_) (`self.HitClassique` _tilecible `Damage?` true))
  (`self.MoveToAtkPlayer` _findenemy_ `Damage?` RefTile _tileennemi))

(fn `AttackClassique`
  (params (RefTile :type Integer))
  (returns (TileCible :type "Array of Integer"))
  (locals (RefeeTile :type Integer) (TileAttack :type "Array of Integer"))
  (set `local.RefeeTile` RefTile)
  (`KismetArrayLibrary.Array_Add` (`local.TileAttack`) (+ (`local.RefeeTile`) 2))
  (`KismetArrayLibrary.Array_Add` (`local.TileAttack`) (+ (`local.RefeeTile`) 3))
  (`KismetArrayLibrary.Array_Add` (`local.TileAttack`) (+ (`local.RefeeTile`) 4))
  (`KismetArrayLibrary.Array_Add` (`local.TileAttack`) (+ (`local.RefeeTile`) 5))
  (`KismetArrayLibrary.Array_Add` (`local.TileAttack`) (+ (`local.RefeeTile`) 6))
  (return (`local.TileAttack`)))

(fn `BoostPerso`
  (params (RefTile :type Integer) (`Enrage?` :type Boolean) (`Armure?` :type Boolean) (`How?` :type Integer))
  (locals (LArmure :type Boolean) (LHow :type Integer) (LEnrage :type Boolean))
  ;[0.05 0.05 0.05] Mettre en négatif pour augment
  (set `local.LEnrage` `Enrage?`)
  (set `local.LArmure` `Armure?`)
  (set `local.LHow` `How?`)
  (for _array_element (`/Game/Map/Tiles/BP_TileManager.AllTiles` (`self.TileManager`))
    (if (== (`/Game/Map/Tiles/BP_Tiles.RefTile` _array_element) RefTile)
      (bind (_hitactor _caseoccupee_) (`/Game/Map/Tiles/BP_Tiles.CheckChara` _array_element))
      (switch `/Game/DataTable/Enum/Enum_CheckTile` _caseoccupee_
        (:`NewEnumerator1`
          (if (`local.LEnrage`)
            (bind _asbp_personnage (cast `/Game/Personnage/BP_Personnage` _hitactor :!pure true))
            (`/Game/Personnage/BP_Personnage.AugmentRage` _asbp_personnage false (`local.LHow`))
            (else
              (`/Game/Personnage/BP_Personnage.TakeDamage` _asbp_personnage (`local.LArmure`) (`local.LHow`)))))))))

(fn `Calcul Damage`
  (params (`Rapide?` :type Boolean))
  (returns (Damage :type Integer))
  (if `Rapide?`
    (return (+ (`self.Atk Rapide`) (`self.Rage`)))
    (else
      (return (+ (`self.Atk Puissante`) (`self.Rage`))))))

(fn `DivideBy2`
  (params (GoDivide :type Integer))
  (returns (Divide :type Integer))
  (return (`KismetMathLibrary.Conv_Int64ToInt` (`KismetMathLibrary.Conv_DoubleToInt64` (/ (`KismetMathLibrary.Conv_IntToDouble` GoDivide) 2.0)))))

(fn `HitClassique`
  (params (TileAttaked :type "Array of Integer (by ref)") (`Damage?` :type Boolean) (`Rapide?` :type Boolean))
  (returns (TileEnnemi :type Integer) (`FindEnemy?` :type Boolean))
  (locals (LTileEnnemi :type Integer) (LAtkSpe :type Boolean) (`LFindEnemy?` :type Boolean))
  (bind _tileattack (`/Game/Map/Tiles/BP_TileManager.CheckTileAttack` (`self.TileManager`) TileAttaked))
  (for _array_element (`/Game/Map/Tiles/BP_TileManager.AllTiles` (`self.TileManager`))
    (bind _reftile (`/Game/Map/Tiles/BP_Tiles.RefTile` _array_element))
    (if (== _reftile _tileattack)
      (set `local.LTileEnnemi` _reftile)
      (if `Damage?`
        (bind (_hitactor _caseoccupee_) (`/Game/Map/Tiles/BP_Tiles.CheckChara` _array_element))
        (switch `/Game/DataTable/Enum/Enum_CheckTile` _caseoccupee_
          (:`NewEnumerator0`
            _)
          (:`NewEnumerator1`
            _)
          (:`NewEnumerator2`
            (bind _damage (`self.Calcul Damage` `Rapide?`))
            (bind _asbp_ennemie (cast `/Game/Personnage/Ennemie/BP_Ennemie` _hitactor :!pure true))
            (`/Game/Personnage/Ennemie/BP_Ennemie.Takehit` _asbp_ennemie _damage (`self.Brise Armure?`) (`self.Armure`) (`self.Sang`) (`self.How Sang?`) (`self.Vulnérable?`) (`self.Affaiblissement?`))
            (`/Engine/EditorBlueprintResources/StandardMacros.IsValid` _asbp_ennemie
              (:`Is Valid`
                (`/Game/UI/WB_HPBar.PlayAnimDamage` (`/Game/Personnage/BP_ParentPerso.WB HPBar` _asbp_ennemie) _damage)
                (return (`local.LTileEnnemi`) true)))))
        (return -110 false)
        (else
          (`/Game/Map/Tiles/BP_Tiles.ChangeEtat` _array_element "NewEnumerator3")
          (bind _hitactor_2 (`/Game/Map/Tiles/BP_Tiles.CheckChara` _array_element))
          (bind _damage_2 (`self.Calcul Damage` `Rapide?`))
          (`/Game/UI/WB_HPBar.UpdateBoxDamage` (`/Game/Personnage/BP_ParentPerso.WB HPBar` (cast `/Game/Personnage/Ennemie/BP_Ennemie` _hitactor_2 :!pure true)) "Visible" _damage_2)
          (return (`local.LTileEnnemi`) false)))))
  (return -110 false))

(fn `MoveToAtkPlayer`
  (params (`FindEnemy?` :type Boolean) (`Damage?` :type Boolean) (RefTilePero :type Integer) (RefTileEnnemi :type Integer))
  (if `FindEnemy?`
    (if `Damage?`
      (`/Game/Personnage/BP_Personnage.MoveToAttack` (cast `/Game/Personnage/BP_Personnage` (`self.GetParentActor`) :!pure true) RefTilePero RefTileEnnemi))))

(fn `ResetRage`)

(fn `SetAttack`
  (params (`Atk Rapide` :type Integer) (`Atk Puissante` :type Integer) (Rage :type Integer))
  (set `self.Atk Rapide` `Atk Rapide`)
  (set `self.Atk Puissante` `Atk Puissante`)
  (set `self.Rage` Rage))

(fn `UserConstructionScript`)