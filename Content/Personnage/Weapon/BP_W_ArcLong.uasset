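; Long bow weapon Blueprint for characters, implementing the quick and powerful attack events on a tile-based battlefield.
; CibleOpposee picks a single opposite target by mirroring the attacker's tile index (6 minus it).
; Both events then set the attack, resolve it through HitClassique and pass the hit tile to MoveToAtkPlayer.
; The two attacks are identical, with the quick one also calling HitClassique with Rapide set to false.
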(event `self.AttackPuissante`
  (params (RefTile :type Integer) (`Damage?` :type Boolean) (AtkRapide :type Integer) (AtkPuissante :type Integer) (Rage :type Integer) (EnumWeapon :type "/Game/DataTable/Enum/Enum_Armes Enum" :default "NewEnumerator0"))
  (`self.SetAttack` AtkRapide AtkPuissante Rage)
  (`self.CibleOpposee` RefTile)
  (bind _tileennemi (`self.HitClassique` (`self.Tile Cible`) `Damage?`))
  (`self.MoveToAtkPlayer` `Damage?` RefTile _tileennemi))

(event `self.AttackRapide`
  (params (RefTile :type Integer) (`Damage?` :type Boolean) (AtkRapide :type Integer) (AtkPuissante :type Integer) (Rage :type Integer) (EnumWeapon :type "/Game/DataTable/Enum/Enum_Armes Enum" :default "NewEnumerator0"))
  (`self.SetAttack` AtkRapide AtkPuissante Rage)
  (`self.CibleOpposee` RefTile)
  (bind _tileennemi (`self.HitClassique` (`self.Tile Cible`) `Damage?`))
  (`self.MoveToAtkPlayer` `Damage?` RefTile _tileennemi))

(fn `CibleOpposee`
  (params (RefTilePerso :type Integer))
  (`KismetArrayLibrary.Array_Clear` (`self.Tile Cible`))
  (`KismetArrayLibrary.Array_Add` (`self.Tile Cible`) (- 6 RefTilePerso))
  (return))

(fn `UserConstructionScript`
  (`parent.UserConstructionScript`))