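; BP_W_BHache is a child weapon Blueprint for the "B Hache" axe, adding weakening and armor-break properties to tile-targeted attacks.
; It enables Affaiblissement (weakening) on BeginPlay.
; Its heavy attack (AttackPuissante) sets BriseArmure and scales the Armure value with weapon level before calling the parent attack.
; The quick attack (AttackRapide) passes straight through to the parent.
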(event `self.ReceiveBeginPlay`
  (`parent.ReceiveBeginPlay`)
  (set `self.Affaiblissement?` true))

(event `self.AttackPuissante`
  (params (RefTile :type Integer) (`Damage?` :type Boolean) (AtkRapide :type Integer) (AtkPuissante :type Integer) (Rage :type Integer) (EnumWeapon :type "/Game/DataTable/Enum/Enum_Armes Enum" :default "NewEnumerator0"))
  ;[0.05 0.05 0.05] Atk Puissante
  (`|ExecutionSequence`
    (:`then_0`
      (switch `/Game/DataTable/Enum/Enum_Armes` EnumWeapon
        (:`NewEnumerator2`
          (set `self.Brise Armure?` true)
          (set `self.Armure` 1))
        (:`NewEnumerator11`
          (set `self.Brise Armure?` true)
          (set `self.Armure` 2))))
    (:`then_1`
      (`parent.AttackPuissante` RefTile `Damage?` AtkRapide AtkPuissante Rage EnumWeapon))))

(event `self.AttackRapide`
  (params (RefTile :type Integer) (`Damage?` :type Boolean) (AtkRapide :type Integer) (AtkPuissante :type Integer) (Rage :type Integer) (EnumWeapon :type "/Game/DataTable/Enum/Enum_Armes Enum" :default "NewEnumerator0"))
  ;[0.05 0.05 0.05] Atk Rapide
  (`parent.AttackRapide` RefTile `Damage?` AtkRapide AtkPuissante Rage EnumWeapon))

(fn `UserConstructionScript`
  (`parent.UserConstructionScript`))