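; Dual-axe weapon Blueprint for tile-based combat, extending a parent weapon with quick and power attacks.
; Quick attack strikes twice via HitClassique, then calls MoveToAtkPlayer; without Damage, DoubleAttack previews the target tile and doubled damage on the enemy health bar.
; Power attack runs the parent logic, then adds character Rage according to weapon level.
; AttackLeft and AttackRight add side target tiles using fixed tile-index offsets.
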(event `self.AttackPuissante`
  (params (RefTile :type Integer) (`Damage?` :type Boolean) (AtkRapide :type Integer) (AtkPuissante :type Integer) (Rage :type Integer) (EnumWeapon :type "/Game/DataTable/Enum/Enum_Armes Enum" :default "NewEnumerator0"))
  (bind _asbp_personnage (cast `/Game/Personnage/BP_Personnage` (`self.GetParentActor`) :!pure true))
  ;[0.05 0.05 0.05] Atk Puissante
  (`parent.AttackPuissante` RefTile `Damage?` AtkRapide AtkPuissante Rage EnumWeapon)
  (switch `/Game/DataTable/Enum/Enum_Armes` EnumWeapon
    (:`NewEnumerator5`
      (`/Game/Personnage/BP_Personnage.AugmentRage` _asbp_personnage false 1))
    (:`NewEnumerator14`
      (`/Game/Personnage/BP_Personnage.AugmentRage` _asbp_personnage false 2))))

(event `self.AttackRapide`
  (params (RefTile :type Integer) (`Damage?` :type Boolean) (AtkRapide :type Integer) (AtkPuissante :type Integer) (Rage :type Integer) (EnumWeapon :type "/Game/DataTable/Enum/Enum_Armes Enum" :default "NewEnumerator0"))
  ;[0.05 0.05 0.05] Atk Rapide
  (`self.SetAttack` AtkRapide AtkPuissante Rage)
  (if `Damage?`
    (bind _tilecible (`self.AttackClassique` RefTile))
    (bind (_tileennemi _findenemy_) (`self.HitClassique` _tilecible `Damage?`))
    (bind _tilecible_2 (`self.AttackClassique` RefTile))
    (`self.HitClassique` _tilecible_2 `Damage?`)
    (`self.MoveToAtkPlayer` _findenemy_ `Damage?` RefTile _tileennemi)
    (else
      (bind _tilecible_3 (`self.AttackClassique` RefTile))
      (`self.DoubleAttack` _tilecible_3))))

(fn `AttackLeft`
  (params (RefTile :type Integer))
  (returns (TileCible :type "Array of Integer"))
  (locals (LRefTile :type Integer) (TileAttack :type "Array of Integer"))
  (set `local.LRefTile` RefTile)
  (`KismetArrayLibrary.Array_Add` (`local.TileAttack`) (+ (`local.LRefTile`) 10))
  (return (`local.TileAttack`)))

(fn `AttackRight`
  (params (RefTile :type Integer))
  (returns (TileCible :type "Array of Integer"))
  (locals (TileAttack :type "Array of Integer") (LRefTile :type Integer))
  (set `local.LRefTile` RefTile)
  (`KismetArrayLibrary.Array_Add` (`local.TileAttack`) (- (`local.LRefTile`) 10))
  (return (`local.TileAttack`)))

(fn `DoubleAttack`
  (params (TileAttaked :type "Array of Integer (by ref)") (`Damage?` :type Boolean) (`Rapide?` :type Boolean))
  (returns (TileEnnemi :type Integer))
  (locals (LDouble :type Boolean) (LRefTile :type Integer))
  (bind _tileattack (`/Game/Map/Tiles/BP_TileManager.CheckTileAttack` (`self.TileManager`) TileAttaked))
  (for _array_element (`/Game/Map/Tiles/BP_TileManager.AllTiles` (`self.TileManager`))
    (bind _reftile (`/Game/Map/Tiles/BP_Tiles.RefTile` _array_element))
    (if (== _reftile _tileattack)
      (set `local.LRefTile` _reftile)
      (if `Damage?`
        (bind (_hitactor _caseoccupee_) (`/Game/Map/Tiles/BP_Tiles.CheckChara` _array_element))
        (switch `/Game/DataTable/Enum/Enum_CheckTile` _caseoccupee_
          (:`NewEnumerator0`
            _)
          (:`NewEnumerator1`
            _)
          (:`NewEnumerator2`
            (bind _damage (`self.Calcul Damage` `Rapide?`))
            (bind _asbp_ennemie (cast `/Game/Personnage/Ennemie/BP_Ennemie` _hitactor :!pure true))
            (`/Game/Personnage/Ennemie/BP_Ennemie.Takehit` _asbp_ennemie (`self.DivideBy2` _damage) false 0 false 0 false false false)
            (`/Game/UI/WB_HPBar.PlayAnimDamage` (`/Game/Personnage/Ennemie/BP_Ennemie.WB HPBar` _asbp_ennemie) 0)
            (return (`local.LRefTile`))))
        (return -110)
        (else
          (`/Game/Map/Tiles/BP_Tiles.ChangeEtat` _array_element "NewEnumerator3")
          (bind _hitactor_2 (`/Game/Map/Tiles/BP_Tiles.CheckChara` _array_element))
          (bind _damage_2 (`self.Calcul Damage` `Rapide?`))
          (`/Game/UI/WB_HPBar.UpdateBoxDamage` (`/Game/Personnage/Ennemie/BP_Ennemie.WB HPBar` (cast `/Game/Personnage/Ennemie/BP_Ennemie` _hitactor_2 :!pure true)) "Visible" (* _damage_2 2))
          (return (`local.LRefTile`)))))))

(fn `UserConstructionScript`
  (`parent.UserConstructionScript`))