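; Greatsword (Espadon) weapon for grid-based combat, whose attacks cleave the tiles either side of the target.
; Powerful and quick attacks run the classic hit and move-to-attack, then a tick later strike the tiles at ±10 index via HitEspadon.
; Side enemies take half damage from powerful attacks and a flat 1 from quick ones.
; With Damage false, HitEspadon only highlights the tile and previews halved damage on the HP bar.
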(event `self.AttackPuissante`
  (params (RefTile :type Integer) (`Damage?` :type Boolean) (AtkRapide :type Integer) (AtkPuissante :type Integer) (Rage :type Integer) (EnumWeapon :type "/Game/DataTable/Enum/Enum_Armes Enum" :default "NewEnumerator0"))
  ;[0.05 0.05 0.05] Atk Puissante
  (`self.SetAttack` AtkRapide AtkPuissante Rage)
  (bind _ally_ (`self.CheckAlly?`))
  (bind _tilecible (`self.AtkClassique` RefTile _ally_))
  (bind (_tileennemi _findenemy_) (`self.HitClassique` _tilecible `Damage?` false _ally_))
  (`self.MoveToAtkPlayer` _findenemy_ `Damage?` RefTile _tileennemi)
  (`KismetSystemLibrary.DelayUntilNextTick`)
  (bind _tilecible_2 (`self.AttackLeft` _tileennemi))
  (`self.HitEspadon` _tilecible_2 `Damage?` false true)
  (bind _tilecible_3 (`self.AttackRight` _tileennemi))
  (`self.HitEspadon` _tilecible_3 `Damage?` false true))

(event `self.AttackRapide`
  (params (RefTile :type Integer) (`Damage?` :type Boolean) (AtkRapide :type Integer) (AtkPuissante :type Integer) (Rage :type Integer) (EnumWeapon :type "/Game/DataTable/Enum/Enum_Armes Enum" :default "NewEnumerator0"))
  ;[0.05 0.05 0.05] Atk Rapide
  (`self.SetAttack` AtkRapide AtkPuissante Rage)
  (bind _ally_ (`self.CheckAlly?`))
  (bind _tilecible (`self.AtkClassique` RefTile _ally_))
  (bind (_tileennemi _findenemy_) (`self.HitClassique` _tilecible `Damage?` true _ally_))
  (`self.MoveToAtkPlayer` _findenemy_ `Damage?` RefTile _tileennemi)
  (`KismetSystemLibrary.DelayUntilNextTick`)
  (bind _tilecible_2 (`self.AttackLeft` _tileennemi))
  (`self.HitEspadon` _tilecible_2 `Damage?` true true true)
  (bind _tilecible_3 (`self.AttackRight` _tileennemi))
  (`self.HitEspadon` _tilecible_3 `Damage?` true true true))

(fn `AttackLeft`
  (params (RefTile :type Integer))
  (returns (TileCible :type "Array of Integer"))
  (locals (LRefTile :type Integer) (TileAttack :type "Array of Integer"))
  (set `local.LRefTile` RefTile)
  (`KismetArrayLibrary.Array_Add` (`local.TileAttack`) (+ (`local.LRefTile`) 10))
  (return (`local.TileAttack`)))

(fn `AttackRight`
  (params (RefTile :type Integer))
  (returns (TileCible :type "Array of Integer"))
  (locals (TileAttack :type "Array of Integer") (LRefTile :type Integer))
  (set `local.LRefTile` RefTile)
  (`KismetArrayLibrary.Array_Add` (`local.TileAttack`) (- (`local.LRefTile`) 10))
  (return (`local.TileAttack`)))

(fn `HitEspadon`
  (params (TileAttaked :type "Array of Integer (by ref)") (`Damage?` :type Boolean) (`Rapide?` :type Boolean) (`ReduceDamage?` :type Boolean) (`1DMG?` :type Boolean))
  (returns (TileEnnemi :type Integer))
  (locals (LReduce :type Boolean) (LRefTile :type Integer :default 0) (L1DMG :type Boolean))
  (set `local.LReduce` `ReduceDamage?`)
  (set `local.L1DMG` `1DMG?`)
  (bind _ally_ (`self.CheckAlly?`))
  (bind _tileattack (`/Game/Map/Tiles/BP_TileManager.CheckTileAttack` (`self.TileManager`) TileAttaked _ally_))
  (for _array_element (`/Game/Map/Tiles/BP_TileManager.AllTiles` (`self.TileManager`))
    (bind _reftile (`/Game/Map/Tiles/BP_Tiles.RefTile` _array_element))
    (if (== _reftile _tileattack)
      (set `local.LRefTile` _reftile)
      (if `Damage?`
        (bind (_hitactor _caseoccupee_) (`/Game/Map/Tiles/BP_Tiles.CheckChara` _array_element))
        (switch `/Game/DataTable/Enum/Enum_CheckTile` _caseoccupee_
          (:`NewEnumerator0`
            _)
          (:`NewEnumerator1`
            _)
          (:`NewEnumerator2`
            (if (`local.L1DMG`)
              (bind _asbp_parent_perso (cast `/Game/Personnage/BP_ParentPerso` _hitactor :!pure true))
              (`/Game/Personnage/Ennemie/BP_Ennemie.Takehit` _asbp_parent_perso 1 false 0 false 0 false false false 0 null)
              (`/Game/UI/WB_HPBar.PlayAnimDamage` (`/Game/Personnage/BP_ParentPerso.WB HPBar` _asbp_parent_perso) 1)
              (else
                (bind _damagefinal (`self.Calcul Damage` `Rapide?` `Damage?`))
                (bind _divide (`self.DivideBy2` _damagefinal))
                (`/Game/Personnage/Ennemie/BP_Ennemie.Takehit` _asbp_parent_perso _divide false 0 false 0 false false false 0 null)
                (`/Game/UI/WB_HPBar.PlayAnimDamage` (`/Game/Personnage/BP_ParentPerso.WB HPBar` _asbp_parent_perso) _divide)))
            (return (`local.LRefTile`))))
        (return -110)
        (else
          (`/Game/Map/Tiles/BP_Tiles.ChangeEtat` _array_element "NewEnumerator3")
          (bind _hitactor_2 (`/Game/Map/Tiles/BP_Tiles.CheckChara` _array_element))
          (bind _damagefinal_2 (`self.Calcul Damage` `Rapide?` `Damage?`))
          (`/Game/UI/WB_HPBar.UpdateBoxDamage` (`/Game/Personnage/BP_ParentPerso.WB HPBar` (cast `/Game/Personnage/BP_ParentPerso` _hitactor_2 :!pure true)) "Visible" (`self.DivideBy2` _damagefinal_2))
          (return (`local.LRefTile`)))))))

(fn `UserConstructionScript`
  (`parent.UserConstructionScript`))