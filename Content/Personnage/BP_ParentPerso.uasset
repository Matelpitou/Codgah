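; Base character for allies and enemies in tile-based combat, with empty Die and BonusNation events.
; Class and weapon data tables, chosen by side, supply stats, modular skin meshes and the weapon child actor that executes quick and powerful attacks.
; Takehit resolves armor, bleed and other statuses, then refreshes the HP bar or GameMode team display.
; Attack movement follows a temporary spawned spline via a timeline that toggles animation flags.
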(event `self.ReceiveBeginPlay`
  (bind _weaponr (`self.WeaponR`))
  (`|ExecutionSequence`
    (:`then_0`
      (bind _asbp_skin_perso (cast `/Game/Package/ModularRPGHeroesPolyart/CharacterBP/BP_SkinPerso` (`ChildActorComponent.ChildActor` (`self.SkinPerso`))))
      (set `self.BP Skin Perso` _asbp_skin_perso)
      (bind _asbp_top_down_game_mode (cast `/Game/TopDown/Blueprints/BP_TopDownGameMode` (`GameplayStatics.GetGameMode`)))
      (set `self.GM` _asbp_top_down_game_mode)
      (bind _aswb_hpbar (cast `/Game/UI/WB_HPBar` (`WidgetComponent.GetWidget` (`self.WidgetHPBar`))))
      (set `self.WB HPBar` _aswb_hpbar)
      (`KismetSystemLibrary.Delay` 0.1)
      (set `self.TileManager` (`/Game/TopDown/Blueprints/BP_TopDownGameMode.TileManager` (`self.GM`)))
      (for _array_element (`/Game/Map/Tiles/BP_TileManager.AllTiles` (`self.TileManager`))
        (if (== (`/Game/Map/Tiles/BP_Tiles.RefTile` _array_element) (`self.StartTest`))
          (`self.MoveChara` (+ (`self.K2_GetActorLocation` _array_element) (`self.UpTpChara`))))))
    (:`then_1`
      (if (`self.Ally?`)
        (set `self.DTClasse` "/Game/DataTable/DT_JClasse.DT_JClasse")
        (set `self.DTArme` "/Game/DataTable/DT_JArme.DT_JArme")
        (else
          (set `self.DTClasse` "/Game/DataTable/DT_EClasse.DT_EClasse")
          (set `self.DTArme` "/Game/DataTable/DT_EArme.DT_EArme")))
      (`self.Update Classe Arme`)
      (`self.UpdateCarac` true)
      (set `self.HPActuel` (- (`self.HPActuel`) (`self.StartHit`)))
      (`/Game/UI/WB_HPBar.InitStat` (`self.WB HPBar`) self)
      (`self.InitSkin`)
      (bind _returnvalue (`|GetDataTableRow` "/Game/DataTable/DT_JSkinArme.DT_JSkinArme" (`KismetStringLibrary.Conv_StringToName` (`|GetEnumeratorNameAsString` (`self.Armes`))))
        (:`then`
          (`ChildActorComponent.SetChildActorClass` _weaponr (`.Right_6_8FDABD2C487755ACAFC54FB7E5707A2C` (break `/Game/DataTable/Structure/Struct_SkinArme` _returnvalue)))
          (`SceneComponent.SetVisibility` _weaponr false false))))))

(event `BonusNation`)

(event `AtkPuissante`
  (params (RefTile :type Integer) (`Damage?` :type Boolean))
  ;[0.05 0.05 0.05] Atk Puissante
  (`/Game/Personnage/Weapon/BP_WeaponParent.AttackPuissante` (cast `/Game/Personnage/Weapon/BP_WeaponParent` (`ChildActorComponent.ChildActor` (`self.WeaponR`)) :!pure true) RefTile `Damage?` (`self.AtkRapideActuel`) (`self.AtkPuissanteActuel`) (`self.Rage`) (`self.Armes`)))

(event `AtkRapide`
  (params (RefTile :type Integer) (`Damage?` :type Boolean))
  ;[0.05 0.05 0.05] Atk Rapide
  (`/Game/Personnage/Weapon/BP_WeaponParent.AttackRapide` (cast `/Game/Personnage/Weapon/BP_WeaponParent` (`ChildActorComponent.ChildActor` (`self.WeaponR`)) :!pure true) RefTile `Damage?` (`self.AtkRapideActuel`) (`self.AtkPuissanteActuel`) (`self.Rage`) (`self.Armes`)))

(event `MoveToAttack`
  (params (RefTilePero :type Integer) (RefTileEnnemi :type Integer))
  ;[0.05 0.05 0.05] Move To Attack
  (for _array_element (`/Game/Map/Tiles/BP_TileManager.AllTiles` (`self.TileManager`))
    (bind _reftile (`/Game/Map/Tiles/BP_Tiles.RefTile` _array_element))
    (if (== _reftile RefTilePero)
      (set `self.LocPerso` (`SceneComponent.K2_GetComponentLocation` (`/Game/Map/Tiles/BP_Tiles.DefaultSceneRoot` _array_element)))
      (elif (== _reftile RefTileEnnemi)
        (set `self.LocEnnemi` (- (`SceneComponent.K2_GetComponentLocation` (`/Game/Map/Tiles/BP_Tiles.DefaultSceneRoot` _array_element)) (0.0 50.0 0.0))))))
  (`|ExecutionSequence`
    (:`then_0`
      (`self.AugmentRage` true)
      (`self.MoveAtkSpline` (`self.LocPerso`) (`self.LocEnnemi`) (`self.Ally?`)))
    (:`then_1`
      (`/Game/TopDown/Blueprints/BP_TopDownController.RemoveInput` (cast `/Game/TopDown/Blueprints/BP_TopDownController` (`GameplayStatics.GetPlayerController` 0) :!pure true)))))

(event `Die`
  ;[0.05 0.05 0.05] Die
)

(event `MoveAtkSpline`
  (params (LocPerso :type "Vector Structure") (LocEnnemi :type "Vector Structure") (`Ally?` :type Boolean))
  ;[0.05 0.05 0.05] MoveAtkSpline
  (bind _returnvalue (`|SpawnActorFromClass` "/Game/Personnage/BP_Spline.BP_Spline_C" (`KismetMathLibrary.MakeTransform` LocPerso) "Undefined" "MultiplyWithRoot" null LocEnnemi LocPerso `Ally?` null))
  (bind (_direction _movetrack) (`Timeline|TL_MoveToAttack` :!via `PlayFromStart`)
    (:`Update`
      (bind _spline (`/Game/Personnage/BP_Spline.Spline` _returnvalue))
      (`self.K2_SetActorLocation` (`SplineComponent.GetLocationAtDistanceAlongSpline` _spline (`KismetMathLibrary.Lerp` 0.0 (`SplineComponent.GetSplineLength` _spline) _movetrack) "World")))
    (:`Finished`
      (`self.K2_DestroyActor` _returnvalue))
    (:`EventAnimGo`
      (set `self.Atk?` true))
    (:`EventAnimEnd`
      (set `self.Atk?` false))))

(event `TakeHitAnim`
  ;[0.05 0.05 0.05] TakehitAnim
  (`KismetSystemLibrary.Delay` 0.4)
  (set `self.TakeHit?` true)
  (`KismetSystemLibrary.RetriggerableDelay` 0.75)
  (set `self.TakeHit?` false))

(fn `AugmentRage`
  (params (`Clear?` :type Boolean) (`How?` :type Integer))
  (if `Clear?`
    (set `self.Rage` 0)
    (else
      (set `self.Rage` (+ (`self.Rage`) `How?`))))
  (`/Game/UI/WB_HPBar.UpdateStat` (`self.WB HPBar`))
  (if (`self.Ally?`)
    (for (_ _array_index) (`/Game/Personnage/BP_ManagerPersonnage.Team` (`/Game/TopDown/Blueprints/BP_TopDownGameMode.Team` (`self.GM`)))
      (`/Game/TopDown/Blueprints/BP_TopDownGameMode.UpdateChara` (`self.GM`) _array_index 0)))
  (return))

(fn `DmgBrut`
  (params (Dmg :type Integer))
  (locals (LMoreDamage :type Integer))
  (set `local.LMoreDamage` Dmg)
  (set `self.HPActuel` (`KismetMathLibrary.Clamp` (- (`self.HPActuel`) (`local.LMoreDamage`)) 0 (`self.HPMax`)))
  (if (<= (`self.HPActuel`) 0)
    (`self.Die`))
  (return))

(fn `HealPerso`
  (params (How :type Integer))
  (returns (HowFinal :type Integer))
  (locals (DiffHP :type Integer))
  (set `local.DiffHP` (- (`self.HPMax`) (`self.HPActuel`)))
  (set `self.HPActuel` (`KismetMathLibrary.Clamp` (+ (`self.HPActuel`) How) 0 (`self.HPMax`)))
  (return (`local.DiffHP`)))

(fn `InitSkin`
  (locals (LStructClasseSkin :type "/Game/DataTable/Structure/Struct_StuffPerso Structure") (LStructArmeSkin :type "/Game/DataTable/Structure/Struct_StuffPerso Structure") (AllFace :type "Array of SkeletalMesh Object Reference"))
  (bind _allface (`local.AllFace`))
  (bind _returnvalue (`|GetDataTableRow` "/Game/DataTable/DT_StuffPerso.DT_StuffPerso" (`KismetStringLibrary.Conv_StringToName` (`|GetEnumeratorNameAsString` (`self.Classes`))))
    (:`then`
      (set `local.LStructClasseSkin` _returnvalue)
      (bind _returnvalue_2 (`|GetDataTableRow` "/Game/DataTable/DT_StuffPerso.DT_StuffPerso" (`KismetStringLibrary.Conv_StringToName` (`|GetEnumeratorNameAsString` (`self.Armes`))))
        (:`then`
          (set `local.LStructArmeSkin` _returnvalue_2)
          (`StaticMeshComponent.SetStaticMesh` (`/Game/Package/ModularRPGHeroesPolyart/CharacterBP/BP_SkinPerso.Bow` (`self.BP Skin Perso`)) (`.Bow_2_51D938114965CC1F86E355BF3E7A816C` (break `/Game/DataTable/Structure/Struct_StuffPerso` (`local.LStructArmeSkin`))))
          (`StaticMeshComponent.SetStaticMesh` (`/Game/Package/ModularRPGHeroesPolyart/CharacterBP/BP_SkinPerso.Arrow` (`self.BP Skin Perso`)) (`.Arrow_17_FEECADBF457326A9D98CE6AD4CEBF4E4` (break `/Game/DataTable/Structure/Struct_StuffPerso` (`local.LStructArmeSkin`))))
          (`StaticMeshComponent.SetStaticMesh` (`/Game/Package/ModularRPGHeroesPolyart/CharacterBP/BP_SkinPerso.LeftWeapon` (`self.BP Skin Perso`)) (`.LeftWeapon_18_7637837B41E5812FE8043181FE0F4D5B` (break `/Game/DataTable/Structure/Struct_StuffPerso` (`local.LStructArmeSkin`))))
          (`StaticMeshComponent.SetStaticMesh` (`/Game/Package/ModularRPGHeroesPolyart/CharacterBP/BP_SkinPerso.RightWeapon` (`self.BP Skin Perso`)) (`.RightWeapon_21_57A8355D43CE424EBAA2E08A315BEAED` (break `/Game/DataTable/Structure/Struct_StuffPerso` (`local.LStructArmeSkin`))))
          (`StaticMeshComponent.SetStaticMesh` (`/Game/Package/ModularRPGHeroesPolyart/CharacterBP/BP_SkinPerso.Shield` (`self.BP Skin Perso`)) (`.Shield_22_D74509D448C7D97A62482FAE125D7837` (break `/Game/DataTable/Structure/Struct_StuffPerso` (`local.LStructArmeSkin`))))
          (`SkeletalMeshComponent.SetSkeletalMeshAsset` (`/Game/Package/ModularRPGHeroesPolyart/CharacterBP/BP_SkinPerso.ShoulderPad` (`self.BP Skin Perso`)) (`.ShoulderPad_28_1E9958594CE9DC85DF44D3BE1E2CCB8A` (break `/Game/DataTable/Structure/Struct_StuffPerso` (`local.LStructClasseSkin`))))
          (`SkeletalMeshComponent.SetSkeletalMeshAsset` (`/Game/Package/ModularRPGHeroesPolyart/CharacterBP/BP_SkinPerso.Shoe` (`self.BP Skin Perso`)) (`.Shoe_5_C2996463490202B04E240D9DFE22C7E5` (break `/Game/DataTable/Structure/Struct_StuffPerso` (`local.LStructClasseSkin`))))
          (`SkeletalMeshComponent.SetSkeletalMeshAsset` (`/Game/Package/ModularRPGHeroesPolyart/CharacterBP/BP_SkinPerso.Glove` (`self.BP Skin Perso`)) (`.Glove_32_9379FECE48329D66E906E18235564C3C` (break `/Game/DataTable/Structure/Struct_StuffPerso` (`local.LStructClasseSkin`))))
          (`SkeletalMeshComponent.SetSkeletalMeshAsset` (`SkeletalMeshActor.SkeletalMeshComponent` (`self.BP Skin Perso`)) (`.Cloth_36_EE14182C4ABB9DB032E85297695D3939` (break `/Game/DataTable/Structure/Struct_StuffPerso` (`local.LStructClasseSkin`))))
          (`SkeletalMeshComponent.SetSkeletalMeshAsset` (`/Game/Package/ModularRPGHeroesPolyart/CharacterBP/BP_SkinPerso.Face` (`self.BP Skin Perso`)) (`|GetArrayItem` _allface (`KismetMathLibrary.RandomIntegerInRange` 0 (- (`KismetArrayLibrary.Array_Length` _allface) 1))))
          (if (`self.Ally?`)
            (bind _returnvalue_3 (`|GetDataTableRow` "/Game/DataTable/DT_StuffPerso.DT_StuffPerso" "Ally")
              (:`then`
                (bind (_bow _arrow _leftweapon _backpack _rightweapon _shield _shoulderpad _belt) (break `/Game/DataTable/Structure/Struct_StuffPerso` _returnvalue_3))
                (`StaticMeshComponent.SetStaticMesh` (`/Game/Package/ModularRPGHeroesPolyart/CharacterBP/BP_SkinPerso.Backpack` (`self.BP Skin Perso`)) _backpack)
                (`SkeletalMeshComponent.SetSkeletalMeshAsset` (`/Game/Package/ModularRPGHeroesPolyart/CharacterBP/BP_SkinPerso.Belt` (`self.BP Skin Perso`)) _belt)
                (`SkeletalMeshComponent.SetSkeletalMeshAsset` (`/Game/Package/ModularRPGHeroesPolyart/CharacterBP/BP_SkinPerso.HeadGears` (`self.BP Skin Perso`)) null)))
            (else
              (`SkeletalMeshComponent.SetSkeletalMeshAsset` (`/Game/Package/ModularRPGHeroesPolyart/CharacterBP/BP_SkinPerso.Hair` (`self.BP Skin Perso`)) "/Game/Package/ModularRPGHeroesPolyart/Meshes/ModularBodyParts/Hair03HalfSK.Hair03HalfSK")
              (`SkeletalMeshComponent.SetSkeletalMeshAsset` (`/Game/Package/ModularRPGHeroesPolyart/CharacterBP/BP_SkinPerso.HeadGears` (`self.BP Skin Perso`)) (`.HeadGears_30_F345944D4B536C7FACE861AADDABB308` (break `/Game/DataTable/Structure/Struct_StuffPerso` (`local.LStructArmeSkin`))))
              (`StaticMeshComponent.SetStaticMesh` (`/Game/Package/ModularRPGHeroesPolyart/CharacterBP/BP_SkinPerso.Backpack` (`self.BP Skin Perso`)) null)
              (`SkeletalMeshComponent.SetSkeletalMeshAsset` (`/Game/Package/ModularRPGHeroesPolyart/CharacterBP/BP_SkinPerso.Belt` (`self.BP Skin Perso`)) null)))
          (`/Game/Package/ModularRPGHeroesPolyart/CharacterBP/BP_SkinPerso.UpdateSkin` (`self.BP Skin Perso`))
          (return))))))

(fn `ModifCarac`
  (params (StatChanges :type "/Game/DataTable/Enum/Enum_Caracteristiques Enum" :default "NewEnumerator0") (How :type Integer))
  (locals (LHow :type Integer))
  (set `local.LHow` How)
  (switch `/Game/DataTable/Enum/Enum_Caracteristiques` StatChanges
    (:`NewEnumerator0`
      (set `self.HPMax` (+ (`self.HPMax`) (`local.LHow`))))
    (:`NewEnumerator1`
      (set `self.HPActuel` (`KismetMathLibrary.Clamp` (+ (`self.HPActuel`) (`local.LHow`)) 0 (`self.HPMax`))))
    (:`NewEnumerator2`
      (set `self.ArmureMax` (+ (`self.ArmureMax`) (`local.LHow`))))
    (:`NewEnumerator3`
      (set `self.ArmureActuel` (`KismetMathLibrary.Clamp` (+ (`self.ArmureActuel`) (`local.LHow`)) 0 (`self.ArmureMax`))))
    (:`NewEnumerator4`
      (set `self.AtkRapideBase` (+ (`self.AtkRapideBase`) (`local.LHow`))))
    (:`NewEnumerator5`
      (set `self.AtkRapideActuel` (+ (`self.AtkRapideActuel`) (`local.LHow`))))
    (:`NewEnumerator6`
      (set `self.AtkPuissanteBase` (+ (`self.AtkPuissanteBase`) (`local.LHow`))))
    (:`NewEnumerator7`
      (set `self.AtkPuissanteActuel` (+ (`self.AtkPuissanteActuel`) (`local.LHow`))))))

(fn `MoveChara`
  (params (Location :type "Vector Structure"))
  (`self.K2_SetActorLocation` Location))

(fn `RecupTile`
  (returns (RefTile :type Integer))
  (bind _returnvalue (`self.K2_GetActorLocation`))
  (bind _outhit (`KismetSystemLibrary.LineTraceSingleByProfile` _returnvalue (- _returnvalue (0.0 0.0 75.0)) "BP_Tiles"))
  (bind _asbp_tiles (cast `/Game/Map/Tiles/BP_Tiles` (`.HitActor` (`GameplayStatics.BreakHitResult` _outhit))))
  (return (`/Game/Map/Tiles/BP_Tiles.RefTile` _asbp_tiles)))

(fn `ReduceSang`
  (params (`AllBlood?` :type Boolean) (`How?` :type Integer))
  (if `AllBlood?`
    (set `self.Sang` 0)
    (else
      (set `self.Sang` (`KismetMathLibrary.Clamp` (- (`self.Sang`) `How?`) 0 1000))))
  (return))

(fn `ResetCarac`
  (set `self.HPMax` 0)
  (set `self.HPActuel` 0)
  (set `self.ArmureMax` 0)
  (set `self.ArmureActuel` 0)
  (set `self.AtkRapideBase` 0)
  (set `self.AtkRapideActuel` 0)
  (set `self.AtkPuissanteBase` 0)
  (set `self.AtkPuissanteActuel` 0))

(fn `Take Damage Sang`
  (params (`ClearBlood?` :type Boolean))
  (bind _sang (`self.Sang`))
  (bind _wb_hpbar (`self.WB HPBar`))
  (if `ClearBlood?`
    (`self.ReduceSang` true)
    (elif (!= _sang 0)
      (`self.Takehit` _sang)
      (`/Game/UI/WB_HPBar.PlayAnimDamage` _wb_hpbar _sang)
      (`self.ReduceSang` false 1)))
  (`/Game/UI/WB_HPBar.UpdateStat` _wb_hpbar)
  (return))

(fn `TakeDamage`
  (params (`BriseArmure?` :type Boolean) (Damage :type Integer))
  (locals (LDamage :type Integer) (LMoreDamage :type Integer))
  (bind _returnvalue (- (`self.ArmureActuel`) (`local.LDamage`)))
  (set `local.LDamage` Damage)
  (if `BriseArmure?`
    (set `self.ArmureActuel` (`KismetMathLibrary.Clamp` (- (`self.ArmureActuel`) (`local.LDamage`)) 0 (`self.ArmureMax`)))
    (return)
    (else
      (set `local.LMoreDamage` _returnvalue)
      (set `self.ArmureActuel` (`KismetMathLibrary.Clamp` _returnvalue 0 (`self.ArmureMax`)))
      (if (<= (`local.LMoreDamage`) 0)
        (set `self.HPActuel` (`KismetMathLibrary.Clamp` (- (`self.HPActuel`) (`KismetMathLibrary.Abs_Int` (`local.LMoreDamage`))) 0 (`self.HPMax`))))
      (if (<= (`self.HPActuel`) 0)
        ;[1 0 0] Add die
        (`self.Die`))
      (return))))

(fn `Takehit`
  (params (Damage :type Integer) (`BriseArmure?` :type Boolean) (Armure :type Integer) (Sang :type Boolean) (`HowSang?` :type Integer) (`Vulnérable?` :type Boolean) (`Affaiblissement?` :type Boolean) (`Epine?` :type Boolean) (HowEpine :type Integer) (Ennemi :type "/Game/Personnage/BP_ParentPerso Object Reference"))
  (returns (DamageDeal :type Integer))
  (locals (LDamage :type Integer) (`LSang?` :type Boolean) (LHowSang :type Integer) (`LVulnerable?` :type Boolean) (`LAffaiblissement?` :type Boolean) (`LBriseArmure?` :type Boolean) (LArmure :type Integer) (`LEpine?` :type Boolean) (LHowEpine :type Integer) (LEnnemie :type "/Game/Personnage/BP_ParentPerso Object Reference"))
  (bind _ldamage (`local.LDamage`))
  (set `local.LDamage` Damage)
  (set `local.LSang?` Sang)
  (set `local.LHowSang` `HowSang?`)
  (set `local.LVulnerable?` `Vulnérable?`)
  (set `local.LAffaiblissement?` `Affaiblissement?`)
  (set `local.LBriseArmure?` `BriseArmure?`)
  (set `local.LEpine?` `Epine?`)
  (set `local.LHowEpine` HowEpine)
  (set `local.LArmure` Armure)
  (set `local.LEnnemie` Ennemi)
  (if (>= (`local.LDamage`) 0)
    (if (`self.Renforce`)
      (set `self.Renforce` false)
      (set `local.LDamage` 0)
      (else
        ;[0.05 0.05 0.05] Epine
        (if (`local.LEpine?`)
          (`self.TakeDamage` (`local.LEnnemie`) false (`local.LHowEpine`))
          (else
            ;[0.05 0.05 0.05] Vulnerable
            (if (`self.Vulnerable`)
              (set `local.LDamage` (`KismetMathLibrary.Round` (* (`KismetMathLibrary.Conv_IntToDouble` (`local.LDamage`)) 1.5)))
              (set `self.Vulnerable` false))
            ;[0.05 0.05 0.05] Brise Armure
            (if (`local.LBriseArmure?`)
              (`self.TakeDamage` true (`local.LArmure`))
              (`self.TakeDamage` false (`local.LDamage`))
              (else
                (`self.TakeDamage` false (`local.LDamage`))))
            ;[0.05 0.05 0.05] Sang
            (if (`local.LSang?`)
              (set `self.Sang` (+ (`local.LHowSang`) (`self.Sang`))))
            ;[0.05 0.05 0.05] Vulnerable
            (if (`local.LVulnerable?`)
              (set `self.Vulnerable` true))
            ;[0.05 0.05 0.05] Affaiblissement
            (if (`local.LAffaiblissement?`)
              (set `self.Affaiblissement` true))))))
    (else
      ;[0.05 0.05 0.05] Heal
      (`self.TakeDamage` false (`local.LDamage`))))
  ;[1 1 1] Modif
  (if (`self.Ally?`)
    (bind _asbp_personnage (cast `/Game/Personnage/BP_Personnage` self)
      (:`then`
        (`KismetSystemLibrary.PrintString` (`KismetStringLibrary.Conv_IntToString` _ldamage))
        (`/Game/TopDown/Blueprints/BP_TopDownGameMode.UpdateChara` (`self.GM`) (`KismetArrayLibrary.Array_Find` (`/Game/Personnage/BP_ManagerPersonnage.Team` (`/Game/TopDown/Blueprints/BP_TopDownGameMode.Team` (`self.GM`))) _asbp_personnage) _ldamage)
        (`self.TakeHitAnim` :!label _label)
        (return (`local.LDamage`)))
      (:`CastFailed`
        (`KismetSystemLibrary.PrintString` "Perso pas dans la team")))
    (else
      (`/Game/UI/WB_HPBar.UpdateStat` (`self.WB HPBar`))
      (goto _label))))

(fn `TakeHitEpine`)

(fn `Update Classe Arme`
  (locals (LStructClasse :type "/Game/DataTable/Structure/Struct_Classes Structure") (LStructArme :type "/Game/DataTable/Structure/Struct_Armes Structure"))
  (bind (_hp _armure _atkrapide _atkpuissante _tswitch _iperso _tclasse) (break `/Game/DataTable/Structure/Struct_Classes` (`local.LStructClasse`)))
  (bind (_hp_2 _armure_2 _atkrapide_2 _atkpuissante_2) (break `/Game/DataTable/Structure/Struct_Classes` (`local.LStructClasse`)))
  (bind (_hp_3 _armure_3 _atkrapide_3 _atkpuissante_3 _tatkrapide _tatkpuissante _tarme) (break `/Game/DataTable/Structure/Struct_Armes` (`local.LStructArme`)))
  (bind (_hp_4 _armure_4 _atkrapide_4 _atkpuissante_4) (break `/Game/DataTable/Structure/Struct_Armes` (`local.LStructArme`)))
  (bind _returnvalue (`|GetDataTableRow` (`self.DTClasse`) (`KismetStringLibrary.Conv_StringToName` (`|GetEnumeratorNameAsString` (`self.Classes`))))
    (:`then`
      (set `local.LStructClasse` _returnvalue)
      (bind _returnvalue_2 (`|GetDataTableRow` (`self.DTArme`) (`KismetStringLibrary.Conv_StringToName` (`|GetEnumeratorNameAsString` (`self.Armes`))))
        (:`then`
          (set `local.LStructArme` _returnvalue_2)
          (set `self.HPMax` (+ _hp_2 _hp_4))
          (set `self.ArmureMax` (+ _armure_2 _armure_4))
          (set `self.AtkRapideBase` (+ _atkrapide_2 _atkrapide_4))
          (set `self.AtkPuissanteBase` (+ _atkpuissante_2 _atkpuissante_4))
          (set `self.TSwitch` _tswitch)
          (set `self.IPerso` _iperso)
          (set `self.TClasse` _tclasse)
          (set `self.TAtkRapide` _tatkrapide)
          (set `self.TAtkPuissante` _tatkpuissante)
          (set `self.TArme` _tarme)
          (if (`self.Ally?`)
            (`self.BonusNation`))
          (return))))))

(fn `UpdateCarac`
  (params (`HP?` :type Boolean))
  (if `HP?`
    (`self.ModifCarac` "NewEnumerator1" (`self.HPMax`)))
  (`self.ModifCarac` "NewEnumerator3" (`self.ArmureMax`))
  (`self.ModifCarac` "NewEnumerator5" (`self.AtkRapideBase`))
  (`self.ModifCarac` "NewEnumerator7" (`self.AtkPuissanteBase`))
  (return))

(fn `UserConstructionScript`)