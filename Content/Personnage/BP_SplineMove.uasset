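; BP_SplineMove is a Blueprint that shapes a three-point spline path between two world locations, LocP1 and LocP2.
; On BeginPlay it pins the end points to those locations and places the middle point at their horizontal midpoint, slightly above LocP1's height.
; When the Right flag is set, the middle point is raised further for a higher arc.
; The graph only builds the path and moves nothing along it.
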(event `self.ReceiveBeginPlay`
  (bind (_locp2_x _locp2_y) (`KismetMathLibrary.BreakVector` (`self.LocP2`)))
  (bind (_locp1_x _locp1_y _locp1_z) (`KismetMathLibrary.BreakVector` (`self.LocP1`)))
  (`SplineComponent.SetLocationAtSplinePoint` (`self.Spline`) 0 (`self.LocP1`) "World" true)
  (`SplineComponent.SetLocationAtSplinePoint` (`self.Spline`) 2 (`self.LocP2`) "World" true)
  (set `self.LocMid` (`KismetMathLibrary.MakeVector` (/ (+ _locp1_x _locp2_x) 2.0) (/ (+ _locp1_y _locp2_y) 2.0) (+ _locp1_z 25.0)))
  (`SplineComponent.SetLocationAtSplinePoint` (`self.Spline`) 1 (`self.LocMid`) "World" true)
  (if (`self.Right?`)
    (set `self.LocMid` (+ (`self.LocMid`) (0.0 0.0 100.0))))
  (`SplineComponent.SetLocationAtSplinePoint` (`self.Spline`) 1 (`self.LocMid`) "World" true))

(fn `UserConstructionScript`)