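; BP_Ennemie is a grid-based enemy character that registers with the enemy manager and fights the player's side and convoy cart.
; PreAction reserves a shuffled, free orthogonal tile within its nine-tile zone and spawns a telegraph arrow.
; Action moves there if still empty, then calls AtkPuissante.
; AtkConvoi damages the cart by column, except for two weapon types, while Die unregisters the enemy and scales its skin through a dissolve timeline before destruction.
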(event `self.ReceiveBeginPlay`
  (`parent.ReceiveBeginPlay`)
  (`self.K2_SetActorRotation` (struct :`Yaw` 180.0))
  (`KismetArrayLibrary.Array_Add` (`/Game/Personnage/Ennemie/BP_EnnemieManager.AllEnnemie` (`/Game/TopDown/Blueprints/BP_TopDownGameMode.ManagerEnnemie` (`self.GM`))) self))

(event `PreAction`
  (bind (_returnvalue_x _returnvalue_y _returnvalue_z) (`KismetMathLibrary.BreakVector` (`self.K2_GetActorLocation`)))
  ;[0.05 0.05 0.05] Pre Action
  (bind _reftile (`self.RecupTile`))
  (bind _tilemove (`self.CheckCroix` _reftile))
  (if (!= (`KismetArrayLibrary.Array_Length` _tilemove) 0)
    (for _array_element _tilemove
      (set `self.TileToAtk` _array_element)
      (for _array_element_2 (`/Game/Map/Tiles/BP_TileManager.AllTiles` (`self.TileManager`)) :!label _label
        (bind _reftile_2 (`/Game/Map/Tiles/BP_Tiles.RefTile` _array_element_2))
        (if (== _reftile_2 (`self.TileToAtk`))
          (bind (_hitactor _caseoccupee_) (`/Game/Map/Tiles/BP_Tiles.CheckChara` _array_element_2))
          (switch `/Game/DataTable/Enum/Enum_CheckTile` _caseoccupee_
            (:`NewEnumerator0`
              (if (not (`/Game/Map/Tiles/BP_Tiles.PreMoveEnn?` _array_element_2))
                (set `self.TileToMove` _reftile_2)
                (set `self.WaitAction?` true)
                (break))))))
      (`KismetSystemLibrary.DelayUntilNextTick`)
      (if (`self.WaitAction?`)
        (for _array_element_3 (`/Game/Map/Tiles/BP_TileManager.AllTiles` (`self.TileManager`))
          (if (== (`/Game/Map/Tiles/BP_Tiles.RefTile` _array_element_3) (`self.TileToMove`))
            (set `/Game/Map/Tiles/BP_Tiles.PreMoveEnn?` true _array_element_3)
            (bind (_returnvalue_x_2 _returnvalue_y_2 _returnvalue_z_2) (`KismetMathLibrary.BreakVector` (`self.K2_GetActorLocation` _array_element_3)))
            (bind (_returnvalue_x_3 _returnvalue_y_3 _returnvalue_z_3) (`KismetMathLibrary.BreakVector` (`KismetMathLibrary.MakeVector` (/ (+ _returnvalue_x_2 _returnvalue_x) 2.0) (/ (+ _returnvalue_y_2 _returnvalue_y) 2.0) _returnvalue_z)))
            (bind (_returnvalue_roll _returnvalue_pitch _returnvalue_yaw) (`KismetMathLibrary.BreakRotator` (`KismetMathLibrary.FindLookAtRotation` (`KismetMathLibrary.MakeVector` _returnvalue_x_2 _returnvalue_y_2 _returnvalue_z_2) (`KismetMathLibrary.MakeVector` _returnvalue_x _returnvalue_y _returnvalue_z))))
            (bind _returnvalue (`|SpawnActorFromClass` "/Game/Personnage/Ennemie/BP_Fleche.BP_Fleche_C" (`KismetMathLibrary.MakeTransform` (`KismetMathLibrary.MakeVector` _returnvalue_x_3 _returnvalue_y_3 (+ _returnvalue_z_3 20.0)) (`KismetMathLibrary.MakeRotator` 0.0 0.0 (- _returnvalue_yaw 180.0))) "Undefined" "MultiplyWithRoot" null null))
            (set `self.BP_Fleche` _returnvalue)
            (break)))))
    (else
      (set `self.TileToAtk` (`|GetArrayItem` _tilemove))
      (goto _label))))

(event `Action`
  (bind _bp_fleche (`self.BP_Fleche`))
  ;[0.05 0.05 0.05] Action
  (for _array_element (`/Game/Map/Tiles/BP_TileManager.AllTiles` (`self.TileManager`))
    (if (== (`/Game/Map/Tiles/BP_Tiles.RefTile` _array_element) (`self.TileToMove`))
      (bind (_hitactor _caseoccupee_) (`/Game/Map/Tiles/BP_Tiles.CheckChara` _array_element))
      (switch `/Game/DataTable/Enum/Enum_CheckTile` _caseoccupee_
        (:`NewEnumerator0`
          (`self.MoveChara` (`self.K2_GetActorLocation` _array_element))
          (set `self.WaitAction?` false)
          (bind _reftile (`self.RecupTile`))
          (`self.AtkPuissante` _reftile true)
          (`/Engine/EditorBlueprintResources/StandardMacros.IsValid` _bp_fleche
            (:`Is Valid`
              (`self.K2_DestroyActor` _bp_fleche))))))))

(event `AtkConvoi`
  (bind _armes (`self.Armes`))
  (bind _bpcharette (`/Game/TopDown/Blueprints/BP_TopDownGameMode.BPCharette` (`self.GM`)))
  ;[0.05 0.05 0.05] AtkConvoi
  (if (not (or (`|EnumEquality` _armes "NewEnumerator16") (`|EnumEquality` _armes "NewEnumerator7")))
    (bind _reftile (`self.RecupTile`))
    (bind _colonne (`self.WhichColonne?` _reftile))
    (set `self.LocPerso` (`SceneComponent.K2_GetComponentLocation` (`self.DefaultSceneRoot`)))
    (switch `int` _colonne
      (:`1`
        (set `self.LocEnnemi` (`SceneComponent.K2_GetComponentLocation` (`/Game/Personnage/Charette/BP_Charette.SphereC1` _bpcharette))))
      (:`2`
        (set `self.LocEnnemi` (`SceneComponent.K2_GetComponentLocation` (`/Game/Personnage/Charette/BP_Charette.SphereC2` _bpcharette))))
      (:`3`
        (set `self.LocEnnemi` (`SceneComponent.K2_GetComponentLocation` (`/Game/Personnage/Charette/BP_Charette.SphereC3` _bpcharette)))))
    (`/Game/Personnage/Charette/BP_Charette.TakeDamage` (`/Game/TopDown/Blueprints/BP_TopDownGameMode.BPCharette` (`self.GM`)) 1)
    (`|ExecutionSequence`
      (:`then_0`
        (`self.MoveAtkSpline` (`self.LocPerso`) (`self.LocEnnemi`) (`self.Ally?`)))
      (:`then_1`
        (`/Game/TopDown/Blueprints/BP_TopDownController.RemoveInput` (cast `/Game/TopDown/Blueprints/BP_TopDownController` (`GameplayStatics.GetPlayerController` 0) :!pure true))))))

(event `self.Die`
  (bind _bp_fleche (`self.BP_Fleche`))
  ;[0.05 0.05 0.05] Die
  (`/Game/Personnage/Ennemie/BP_EnnemieManager.EnnemyDie` (`/Game/TopDown/Blueprints/BP_TopDownGameMode.ManagerEnnemie` (`self.GM`)) self)
  (`/Engine/EditorBlueprintResources/StandardMacros.IsValid` _bp_fleche
    (:`Is Valid`
      (`self.K2_DestroyActor` _bp_fleche))
    (:`Is Not Valid`
      _))
  (`parent.Die`)
  (set `self.Die?` true)
  (`PrimitiveComponent.SetCollisionEnabled` (`self.Capsule`) "NoCollision")
  (`KismetSystemLibrary.Delay` 1.5)
  (bind (_direction _dissolve) (`Timeline|TL_Dissolve` :!via `PlayFromStart`)
    (:`Update`
      (`SceneComponent.SetWorldScale3D` (`self.SkinPerso`) (`KismetMathLibrary.Conv_DoubleToVector` _dissolve)))
    (:`Finished`
      (`self.K2_DestroyActor`))))

(fn `CheckCroix`
  (params (RefTile :type Integer))
  (returns (TileMove :type "Array of Integer"))
  (locals (LRefTile :type Integer) (LTileMove :type "Array of Integer"))
  (bind _ltilemove (`local.LTileMove`))
  (bind _returnvalue (+ (`local.LRefTile`) 10))
  (bind _returnvalue_2 (- (`local.LRefTile`) 10))
  (bind _returnvalue_3 (+ (`local.LRefTile`) 1))
  (bind _returnvalue_4 (- (`local.LRefTile`) 1))
  (set `local.LRefTile` RefTile)
  (bind _inrange_ (`self.CheckOwnTile` _returnvalue_3))
  (if _inrange_
    (`KismetArrayLibrary.Array_Add` (`local.LTileMove`) _returnvalue_3))
  (bind _inrange__2 (`self.CheckOwnTile` _returnvalue_4))
  (if _inrange__2
    (`KismetArrayLibrary.Array_Add` (`local.LTileMove`) _returnvalue_4))
  (bind _inrange__3 (`self.CheckOwnTile` _returnvalue))
  (if _inrange__3
    (`KismetArrayLibrary.Array_Add` (`local.LTileMove`) _returnvalue))
  (bind _inrange__4 (`self.CheckOwnTile` _returnvalue_2))
  (if _inrange__4
    (`KismetArrayLibrary.Array_Add` _ltilemove _returnvalue_2))
  (`KismetArrayLibrary.Array_Shuffle` _ltilemove)
  (return _ltilemove))

(fn `CheckOwnTile`
  (params (RefTile :type Integer))
  (returns (`InRange?` :type Boolean))
  (locals (LReftTile :type Integer))
  (bind _lrefttile (`local.LReftTile`))
  (bind _lrefttile_2 (`local.LReftTile`))
  (bind _lrefttile_3 (`local.LReftTile`))
  (set `local.LReftTile` RefTile)
  (return (or (== _lrefttile_2 4) (== _lrefttile_2 5) (== _lrefttile_2 6) (== _lrefttile_3 14) (== _lrefttile_3 15) (== _lrefttile_3 16) (== _lrefttile 24) (== _lrefttile 25) (== _lrefttile 26))))

(fn `DieEnnemie`
  (set `self.Die?` true)
  (`/Game/Package/ModularRPGHeroesPolyart/CharacterBP/BP_SkinPerso.UpdateOutline` (cast `/Game/Package/ModularRPGHeroesPolyart/CharacterBP/BP_SkinPerso` (`ChildActorComponent.ChildActor` (`self.SkinPerso`)) :!pure true) false))

(fn `UserConstructionScript`)

(fn `WhichColonne?`
  (params (RefTile :type Integer))
  (returns (Colonne :type Integer))
  (locals (LLRefTile :type Integer) (LColonne :type Integer))
  (bind _llreftile (`local.LLRefTile`))
  (bind _llreftile_2 (`local.LLRefTile`))
  (bind _llreftile_3 (`local.LLRefTile`))
  (set `local.LLRefTile` RefTile)
  (if (or (== _llreftile_2 4) (== _llreftile_2 5) (== _llreftile_2 6))
    (set `local.LColonne` 1)
    (elif (or (== _llreftile_3 14) (== _llreftile_3 15) (== _llreftile_3 16))
      (set `local.LColonne` 2)
      (elif (or (== _llreftile 24) (== _llreftile 25) (== _llreftile 26))
        (set `local.LColonne` 3)
        (else
          (set `local.LColonne` 0)
          (`KismetSystemLibrary.PrintString` "Ennemi Hors Colonne pour Atk convoi")))))
  (return (`local.LColonne`)))