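; Enemy manager for fights: it registers with the game mode and drives the enemy group's attacks and the end of combat.
; HowAtk shuffles enemies and calls PreAction on one or two, per the tile's DT_FightManager row.
; GoAtkPuissante steps through them recursively with delays, firing Action if waiting, otherwise AtkRapide.
; When all die, it resets the team, heals a member if NumberCorbeau is high enough, flags victory and shows WB_EndFight.
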(event `self.ReceiveBeginPlay`
  (bind _asbp_top_down_game_mode (cast `/Game/TopDown/Blueprints/BP_TopDownGameMode` (`GameplayStatics.GetGameMode`)))
  (set `self.GM` _asbp_top_down_game_mode)
  (set `/Game/TopDown/Blueprints/BP_TopDownGameMode.ManagerEnnemie` self _asbp_top_down_game_mode))

(event `EnnemyDie`
  (params (EnnemieDie :type "/Game/Personnage/Ennemie/BP_Ennemie Object Reference"))
  (bind _allennemie (`self.AllEnnemie`))
  (`KismetArrayLibrary.Array_RemoveItem` _allennemie EnnemieDie)
  (`KismetSystemLibrary.DelayUntilNextTick`)
  (if (<= (`KismetArrayLibrary.Array_Length` _allennemie) 0)
    (for _array_element (`/Game/Personnage/BP_ManagerPersonnage.Team` (`/Game/TopDown/Blueprints/BP_TopDownGameMode.Team` (`self.GM`)))
      (`/Game/Personnage/BP_Personnage.ResetChara` _array_element))
    (`self.EndFight`)))

(event `EndFight`
  (bind _persoaheal (`self.PersoaHeal`))
  (`KismetSystemLibrary.Delay` 0.6)
  (set `self.PersoaHeal` null)
  (if (>= (`/Game/UI/WB_MainAdv.NumberCorbeau` (`/Game/TopDown/Blueprints/BP_TopDownGameMode.WBMainAdv` (`self.GM`))) 6)
    (for _array_element (`/Game/Personnage/BP_ManagerPersonnage.Team` (`/Game/TopDown/Blueprints/BP_TopDownGameMode.Team` (`self.GM`)))
      (`/Engine/EditorBlueprintResources/StandardMacros.IsValid` _array_element
        (:`Is Valid`
          (if (< (`/Game/Personnage/BP_ParentPerso.HPActuel` _array_element) (`/Game/Personnage/BP_ParentPerso.HPActuel` (`self.PersoaHeal`)))
            (set `self.PersoaHeal` _array_element :!label _label)))
        (:`Is Not Valid`
          (goto _label))))
    (`/Engine/EditorBlueprintResources/StandardMacros.IsValid` _persoaheal
      (:`Is Valid`
        (`/Game/Personnage/BP_ParentPerso.Takehit` _persoaheal -3 false 0 false 0 false false false 0 null))
      (:`Is Not Valid`
        _)))
  (`KismetSystemLibrary.Delay` 0.6)
  (for _array_element_2 (`/Game/Personnage/BP_ManagerPersonnage.Team` (`/Game/TopDown/Blueprints/BP_TopDownGameMode.Team` (`self.GM`)))
    (set `/Game/Personnage/BP_ParentPerso.Victoire?` true _array_element_2))
  (`KismetSystemLibrary.Delay` 2.0)
  (bind _returnvalue (`|CreateWidget` "/Game/UI/WB_EndFight.WB_EndFight_C"))
  (`UserWidget.AddToViewport` _returnvalue 0))

(event `HowAtk`
  (bind _output (`|GetArrayItem` (`self.AllEnnemie`) 1))
  (bind _output_2 (`|GetArrayItem` (`self.AllEnnemie`)))
  (bind _output_3 (`|GetArrayItem` (`self.AllEnnemie`)))
  ;[0.05 0.05 0.05] HowAtkPuissante?
  (bind _asbp_tiles_adv (`/Game/Adventure/CharetteAdv/BP_CharetteAdv2.OnWhichTile` (`/Game/TopDown/Blueprints/BP_TopDownGameMode.CharetteAdv` (`self.GM`))))
  (bind _returnvalue (`|GetDataTableRow` "/Game/DataTable/DT_FightManager.DT_FightManager" (`KismetStringLibrary.Conv_StringToName` (`KismetStringLibrary.Conv_IntToString` (`/Game/Adventure/TilesAdv/BP_TilesAdv.RefFight` _asbp_tiles_adv))))
    (:`then`
      (`KismetArrayLibrary.Array_Shuffle` (`self.AllEnnemie`))
      (if (!= (- (`.NbrAtk_44_1DFB542942242E8EEC0E2FA19E87025E` (break `/Game/DataTable/Structure/Struct_ManagerEnnemi` _returnvalue)) 1) 0)
        (`/Engine/EditorBlueprintResources/StandardMacros.IsValid` _output_3
          (:`Is Valid`
            (`/Game/Personnage/Ennemie/BP_Ennemie.PreAction` _output_3))
          (:`Is Not Valid`
            _))
        (`KismetSystemLibrary.Delay` 0.2)
        (`/Engine/EditorBlueprintResources/StandardMacros.IsValid` _output
          (:`Is Valid`
            (`/Game/Personnage/Ennemie/BP_Ennemie.PreAction` _output)))
        (else
          (`/Engine/EditorBlueprintResources/StandardMacros.IsValid` _output_2
            (:`Is Valid`
              (`/Game/Personnage/Ennemie/BP_Ennemie.PreAction` _output_2))))))
    (:`RowNotFound`
      (`KismetSystemLibrary.PrintString` "Hello"))))

(event `LoopAtkPuissante`
  (bind _checktableau (`self.CheckTableau`))
  (bind _allennemie (`self.AllEnnemie`))
  (bind _output (`|GetArrayItem` _allennemie _checktableau))
  ;[0.05 0.05 0.05] Go Atk Puissante
  (set `self.CheckTableau` (+ (`self.CheckTableau`) 1))
  (if (< _checktableau (`KismetArrayLibrary.Array_Length` _allennemie)) :!label _label_2
    (`/Engine/EditorBlueprintResources/StandardMacros.IsValid` _output
      (:`Is Valid`
        (if (`/Game/Personnage/Ennemie/BP_Ennemie.WaitAction?` _output)
          (`/Game/Personnage/Ennemie/BP_Ennemie.Action` _output)
          (else
            (bind _reftile (`/Game/Personnage/BP_ParentPerso.RecupTile` _output))
            (`/Game/Personnage/BP_ParentPerso.AtkRapide` _output _reftile true)))
        (`KismetSystemLibrary.Delay` 0.9)
        (`self.LoopAtkPuissante`)))))

(event `GoAtkPuissante`
  ;[0.05 0.05 0.05] Go Atk Puissante
  (set `self.CheckTableau` 0)
  (goto _label_2))

(fn `UserConstructionScript`)