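; Cart actor with its own health, shown through a WB_HPCharette widget.
; On BeginPlay it registers itself with BP_TopDownGameMode and loads its HP from the Player row of DT_Player.
; TakeDamage subtracts damage, clamps it against that row's maximum and refreshes the widget.
; Each hit replays a timeline that offsets the Charette component along local X, with a retriggerable delay stopping it.
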(event `self.ReceiveBeginPlay`
  (set `self.Relative Location Charette` (`SceneComponent.RelativeLocation` (`self.Charette`)))
  (bind _asbp_top_down_game_mode (cast `/Game/TopDown/Blueprints/BP_TopDownGameMode` (`GameplayStatics.GetGameMode`)))
  (set `/Game/TopDown/Blueprints/BP_TopDownGameMode.BPCharette` self _asbp_top_down_game_mode)
  (bind _aswb_hpcharette (cast `/Game/UI/WB_HPCharette` (`WidgetComponent.GetWidget` (`self.Widget`))))
  (set `self.WBHP Charette` _aswb_hpcharette)
  (bind _returnvalue (`|GetDataTableRow` "/Game/DataTable/DT_Player.DT_Player" "Player")
    (:`then`
      (bind (_speedzoom _minzoom _maxzoom _hpcharette) (break `/Game/DataTable/Structure/Struct_Player` _returnvalue))
      (set `self.HPCharette` _hpcharette)
      (`/Game/UI/WB_HPCharette.UpdateHP` _aswb_hpcharette _hpcharette))))

(event `TakeDamage`
  (params (`How?` :type Integer))
  (bind (_relative_location_charette_x _relative_location_charette_y _relative_location_charette_z) (`KismetMathLibrary.BreakVector` (`self.Relative Location Charette`)))
  (bind _returnvalue (`|GetDataTableRow` "/Game/DataTable/DT_Player.DT_Player" "Player")
    (:`then`
      (set `self.HPCharette` (`KismetMathLibrary.Clamp` (- (`self.HPCharette`) `How?`) 0 (`.HPCharette_10_20FA403C485C02A1D29590A0AFEDAA46` (break `/Game/DataTable/Structure/Struct_Player` _returnvalue))))
      (`/Game/UI/WB_HPCharette.UpdateHP` (`self.WBHP Charette`) (`self.HPCharette`))
      (`|ExecutionSequence`
        (:`then_0`
          (bind (_direction _move) (`Timeline|TL_TakeHit` :!via `PlayFromStart` :!label _label)
            (:`Update`
              (`SceneComponent.K2_SetRelativeLocation` (`self.Charette`) (`KismetMathLibrary.MakeVector` (+ _move _relative_location_charette_x) _relative_location_charette_y _relative_location_charette_z) false false))
            (:`Finished`
              (`SceneComponent.K2_SetRelativeLocation` (`self.Charette`) (`self.Relative Location Charette`) false false))))
        (:`then_1`
          (`KismetSystemLibrary.RetriggerableDelay` 0.4)
          (goto _label :!via `Stop`))))))

(fn `UserConstructionScript`)