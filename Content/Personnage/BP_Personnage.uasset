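; Player character for a tile-based tactical game, with body color and switch pattern (cross, far, around) set by its Nation.
; BeginPlay places it on a tile, sums class and weapon DataTable stats, then initializes its HP bar and hand weapons.
; Deplacement sends move and switch tiles to TileManager, limiting forward ones to hardcoded 3x3 grid indices.
; Attacks delegate to the weapon child actor, while MoveToAttack follows a spawned spline via timeline and removes input.
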(event `self.ReceiveBeginPlay`
  (`|ExecutionSequence`
    (:`then_0`
      (`KismetSystemLibrary.Delay` 0.2)
      (`self.MoveChara` (+ (`self.K2_GetActorLocation` (`|GetArrayItem` (`/Game/Map/Tiles/BP_TileManager.AllTiles` (`self.TileManager`)) (`self.StartTest`))) (`self.UpTpChara`))))
    (:`then_1`
      (switch `/Game/DataTable/Enum/Enum_Nation` (`self.Nation`)
        (:`NewEnumerator0`
          (`PrimitiveComponent.SetMaterial` (`self.SkeletalMesh`) 0 "/Game/Package/CloseCombatAnimSet/Mannequin/Character/Materials/M_UE4Man_BodyRed.M_UE4Man_BodyRed"))
        (:`NewEnumerator1`
          (`PrimitiveComponent.SetMaterial` (`self.SkeletalMesh`) 0 "/Game/Package/CloseCombatAnimSet/Mannequin/Character/Materials/M_UE4Man_BodyGreen.M_UE4Man_BodyGreen"))
        (:`NewEnumerator2`
          (`PrimitiveComponent.SetMaterial` (`self.SkeletalMesh`) 0 "/Game/Package/CloseCombatAnimSet/Mannequin/Character/Materials/M_UE4Man_BodyBlue.M_UE4Man_BodyBlue"))))
    (:`then_2`
      (bind _returnvalue (`|GetDataTableRow` "/Game/DataTable/DT_JClasse.DT_JClasse" (`KismetStringLibrary.Conv_StringToName` (`|GetEnumeratorNameAsString` (`self.Classes`))))
        (:`then`
          (bind (_hp _armure _atkrapide _atkpuissante) (break `/Game/DataTable/Structure/Struct_Classes` _returnvalue))
          (`self.ModifCarac` "NewEnumerator0" _hp)
          (`self.ModifCarac` "NewEnumerator2" _armure)
          (`self.ModifCarac` "NewEnumerator4" _atkrapide)
          (`self.ModifCarac` "NewEnumerator6" _atkpuissante)
          (bind _returnvalue_2 (`|GetDataTableRow` "/Game/DataTable/DT_JArme.DT_JArme" (`KismetStringLibrary.Conv_StringToName` (`|GetEnumeratorNameAsString` (`self.Armes`))))
            (:`then`
              (bind (_hp_2 _armure_2 _atkrapide_2 _atkpuissante_2) (break `/Game/DataTable/Structure/Struct_Armes` _returnvalue_2))
              (`self.ModifCarac` "NewEnumerator0" _hp_2)
              (`self.ModifCarac` "NewEnumerator2" _armure_2)
              (`self.ModifCarac` "NewEnumerator4" _atkrapide_2)
              (`self.ModifCarac` "NewEnumerator6" _atkpuissante_2)
              (`self.ModifCarac` "NewEnumerator1" (`self.HPMax`))
              (`self.ModifCarac` "NewEnumerator3" (`self.ArmureMax`))
              (`self.ModifCarac` "NewEnumerator5" (`self.AtkRapideBase`))
              (`self.ModifCarac` "NewEnumerator7" (`self.AtkPuissanteBase`))
              (bind _aswb_hpbar (cast `/Game/UI/WB_HPBar` (`WidgetComponent.GetWidget` (`self.WidgetHPBar`))))
              (set `self.WB HPBar` _aswb_hpbar)
              (`/Game/UI/WB_HPBar.Init` _aswb_hpbar self null true)
              (bind _returnvalue_3 (`|GetDataTableRow` "/Game/DataTable/DT_JSkinArme.DT_JSkinArme" (`KismetStringLibrary.Conv_StringToName` (`|GetEnumeratorNameAsString` (`self.Armes`))))
                (:`then`
                  (bind (_right _left) (break `/Game/DataTable/Structure/Struct_SkinArme` _returnvalue_3))
                  (`ChildActorComponent.SetChildActorClass` (`self.WeaponR`) _right)
                  (`SceneComponent.K2_AttachToComponent` (`self.WeaponR`) (`self.SkeletalMesh`) "hand_rSocket" "SnapToTarget" "SnapToTarget" "KeepRelative" true)
                  (`/Engine/EditorBlueprintResources/StandardMacros.IsValid` _left
                    (:`Is Valid`
                      (`StaticMeshComponent.SetStaticMesh` (`self.WeaponL`) _left)
                      (`SceneComponent.K2_AttachToComponent` (`self.WeaponL`) (`self.SkeletalMesh`) "hand_lSocket" "SnapToTarget" "SnapToTarget" "KeepRelative" true)
                      (`SceneComponent.K2_SetRelativeRotation` (`self.WeaponL`) (struct :`Pitch` 180.0) false false))))))))))))

(event `Deplacement`
  (params (RefTile :type Integer))
  (switch `/Game/DataTable/Enum/Enum_Nation` (`self.Nation`)
    (:`NewEnumerator0`
      (bind _tiletocheck (`self.SwitchCroix` RefTile))
      (bind _tiletocheck_2 (`self.SImpleMove` RefTile))
      (`/Game/Map/Tiles/BP_TileManager.CheckTileMove` (`self.TileManager`) _tiletocheck_2 _tiletocheck))
    (:`NewEnumerator1`
      (bind _tiletocheck_3 (`self.SwitchFar` RefTile))
      (bind _tiletocheck_4 (`self.SImpleMove` RefTile))
      (`/Game/Map/Tiles/BP_TileManager.CheckTileMove` (`self.TileManager`) _tiletocheck_4 _tiletocheck_3))
    (:`NewEnumerator2`
      (bind _tiletocheck_5 (`self.SwitchAround` RefTile))
      (bind _tiletocheck_6 (`self.SImpleMove` RefTile))
      (`/Game/Map/Tiles/BP_TileManager.CheckTileMove` (`self.TileManager`) _tiletocheck_6 _tiletocheck_5))))

(event `AttackPuissantePlayer`
  (params (RefTile :type Integer) (`Damage?` :type Boolean))
  (`/Game/Personnage/Weapon/BP_WeaponParent.AttackPuissante` (cast `/Game/Personnage/Weapon/BP_WeaponParent` (`ChildActorComponent.ChildActor` (`self.WeaponR`)) :!pure true) RefTile `Damage?` (`self.AtkRapideActuel`) (`self.AtkPuissanteActuel`) (`self.Rage`) (`self.Armes`)))

(event `AttackRapidePlayer`
  (params (RefTile :type Integer) (`Damage?` :type Boolean))
  (`/Game/Personnage/Weapon/BP_WeaponParent.AttackRapide` (cast `/Game/Personnage/Weapon/BP_WeaponParent` (`ChildActorComponent.ChildActor` (`self.WeaponR`)) :!pure true) RefTile `Damage?` (`self.AtkRapideActuel`) (`self.AtkPuissanteActuel`) (`self.Rage`) (`self.Armes`)))

(event `MoveToAttack`
  (params (RefTilePero :type Integer) (RefTileEnnemi :type Integer))
  (for _array_element (`/Game/Map/Tiles/BP_TileManager.AllTiles` (`self.TileManager`))
    (bind _reftile (`/Game/Map/Tiles/BP_Tiles.RefTile` _array_element))
    (if (== _reftile RefTilePero)
      (set `self.LocPerso` (`SceneComponent.K2_GetComponentLocation` (`/Game/Map/Tiles/BP_Tiles.DefaultSceneRoot` _array_element)))
      (elif (== _reftile RefTileEnnemi)
        (set `self.LocEnnemi` (`SceneComponent.K2_GetComponentLocation` (`/Game/Map/Tiles/BP_Tiles.DefaultSceneRoot` _array_element))))))
  (`|ExecutionSequence`
    (:`then_0`
      (bind _returnvalue (`|SpawnActorFromClass` "/Game/Personnage/BP_Spline.BP_Spline_C" (`KismetMathLibrary.MakeTransform` (`self.LocPerso`)) "Undefined" "MultiplyWithRoot" null (`self.LocEnnemi`) (`self.LocPerso`) null))
      (bind (_direction _movetrack) (`Timeline|TL_MoveToAttack` :!via `PlayFromStart`)
        (:`Update`
          (bind _spline (`/Game/Personnage/BP_Spline.Spline` _returnvalue))
          (`self.K2_SetActorLocation` (`SplineComponent.GetLocationAtDistanceAlongSpline` _spline (`KismetMathLibrary.Lerp` 0.0 (`SplineComponent.GetSplineLength` _spline) _movetrack) "World")))
        (:`Finished`
          (`self.K2_DestroyActor` _returnvalue))))
    (:`then_1`
      (`/Game/TopDown/Blueprints/BP_TopDownController.RemoveInput` (cast `/Game/TopDown/Blueprints/BP_TopDownController` (`GameplayStatics.GetPlayerController` 0) :!pure true)))))

(fn `Attack`
  (params (RefTile :type Integer))
  (returns (TileAttack1 :type "Array of Integer"))
  (locals (TileAttack :type "Array of Integer") (RefeeTile :type Integer))
  (set `local.RefeeTile` RefTile)
  (`KismetArrayLibrary.Array_Add` (`local.TileAttack`) (+ (`local.RefeeTile`) 2))
  (`KismetArrayLibrary.Array_Add` (`local.TileAttack`) (+ (`local.RefeeTile`) 3))
  (`KismetArrayLibrary.Array_Add` (`local.TileAttack`) (+ (`local.RefeeTile`) 4))
  (`KismetArrayLibrary.Array_Add` (`local.TileAttack`) (+ (`local.RefeeTile`) 5))
  (`KismetArrayLibrary.Array_Add` (`local.TileAttack`) (+ (`local.RefeeTile`) 6))
  (return (`local.TileAttack`)))

(fn `CheckOwnTile`
  (params (RefTile :type Integer))
  (returns (`AddTile?` :type Boolean))
  (locals (AllTile :type "Array of Integer"))
  (return (or (== RefTile 0) (== RefTile 1) (== RefTile 2) (== RefTile 10) (== RefTile 11) (== RefTile 12) (== RefTile 20) (== RefTile 21) (== RefTile 22))))

(fn `ModifCarac`
  (params (StatChanges :type "/Game/DataTable/Enum/Enum_Caracteristiques Enum" :default "NewEnumerator0") (How :type Integer))
  (locals (LHow :type Integer))
  (set `local.LHow` How)
  (switch `/Game/DataTable/Enum/Enum_Caracteristiques` StatChanges
    (:`NewEnumerator0`
      (set `self.HPMax` (+ (`self.HPMax`) (`local.LHow`))))
    (:`NewEnumerator1`
      (set `self.HPActuel` (`KismetMathLibrary.Clamp` (+ (`self.HPActuel`) (`local.LHow`)) 0 (`self.HPMax`))))
    (:`NewEnumerator2`
      (set `self.ArmureMax` (+ (`self.ArmureMax`) (`local.LHow`))))
    (:`NewEnumerator3`
      (set `self.ArmureActuel` (`KismetMathLibrary.Clamp` (+ (`self.ArmureActuel`) (`local.LHow`)) 0 (`self.ArmureMax`))))
    (:`NewEnumerator4`
      (set `self.AtkRapideBase` (+ (`self.AtkRapideBase`) (`local.LHow`))))
    (:`NewEnumerator5`
      (set `self.AtkRapideActuel` (+ (`self.AtkRapideActuel`) (`local.LHow`))))
    (:`NewEnumerator6`
      (set `self.AtkPuissanteBase` (+ (`self.AtkPuissanteBase`) (`local.LHow`))))
    (:`NewEnumerator7`
      (set `self.AtkPuissanteActuel` (+ (`self.AtkPuissanteActuel`) (`local.LHow`))))))

(fn `MoveChara`
  (params (Location :type "Vector Structure"))
  (`self.K2_SetActorLocation` Location))

(fn `SImpleMove`
  (params (RefTile :type Integer))
  (returns (TileToCheck :type "Array of Integer"))
  (locals (TileCheck :type "Array of Integer") (RefeTile :type Integer))
  (bind _returnvalue (+ (`local.RefeTile`) 1))
  (set `local.RefeTile` RefTile)
  (`KismetArrayLibrary.Array_Add` (`local.TileCheck`) (- (`local.RefeTile`) 1))
  (`KismetArrayLibrary.Array_Add` (`local.TileCheck`) (+ (`local.RefeTile`) 10))
  (`KismetArrayLibrary.Array_Add` (`local.TileCheck`) (- (`local.RefeTile`) 10))
  (if (or (== _returnvalue 0) (== _returnvalue 1) (== _returnvalue 2) (== _returnvalue 10) (== _returnvalue 11) (== _returnvalue 12) (== _returnvalue 20) (== _returnvalue 21) (== _returnvalue 22))
    (`KismetArrayLibrary.Array_Add` (`local.TileCheck`) _returnvalue))
  (return (`local.TileCheck`)))

(fn `SwitchAround`
  (params (RefTile :type Integer))
  (returns (TileToCheck :type "Array of Integer"))
  (locals (TileCheck :type "Array of Integer") (RefeTile :type Integer))
  (bind _returnvalue (+ (`local.RefeTile`) 1))
  (bind _returnvalue_2 (+ (`local.RefeTile`) 11))
  (bind _returnvalue_3 (- (`local.RefeTile`) 9))
  (set `local.RefeTile` RefTile)
  (`KismetArrayLibrary.Array_Add` (`local.TileCheck`) (- (`local.RefeTile`) 1))
  (`KismetArrayLibrary.Array_Add` (`local.TileCheck`) (- (`local.RefeTile`) 11))
  (`KismetArrayLibrary.Array_Add` (`local.TileCheck`) (+ (`local.RefeTile`) 9))
  (`KismetArrayLibrary.Array_Add` (`local.TileCheck`) (+ (`local.RefeTile`) 10))
  (`KismetArrayLibrary.Array_Add` (`local.TileCheck`) (- (`local.RefeTile`) 10))
  (bind _addtile_ (`self.CheckOwnTile` _returnvalue))
  (if _addtile_
    (`KismetArrayLibrary.Array_Add` (`local.TileCheck`) _returnvalue))
  (bind _addtile__2 (`self.CheckOwnTile` _returnvalue_2))
  (if _addtile__2
    (`KismetArrayLibrary.Array_Add` (`local.TileCheck`) _returnvalue_2))
  (bind _addtile__3 (`self.CheckOwnTile` _returnvalue_3))
  (if _addtile__3
    (`KismetArrayLibrary.Array_Add` (`local.TileCheck`) _returnvalue_3))
  (return (`local.TileCheck`)))

(fn `SwitchCroix`
  (params (RefTile :type Integer))
  (returns (TileToCheck :type "Array of Integer"))
  (locals (TileCheck :type "Array of Integer") (RefeTile :type Integer))
  (bind _returnvalue (+ (`local.RefeTile`) 1))
  (bind _returnvalue_2 (+ (`local.RefeTile`) 2))
  (set `local.RefeTile` RefTile)
  ;[0.05 0.05 0.05] Derriere
  (`KismetArrayLibrary.Array_Add` (`local.TileCheck`) (- (`local.RefeTile`) 1))
  (`KismetArrayLibrary.Array_Add` (`local.TileCheck`) (- (`local.RefeTile`) 2))
  ;[0.05 0.05 0.05] Gauche
  (`KismetArrayLibrary.Array_Add` (`local.TileCheck`) (- (`local.RefeTile`) 20))
  (`KismetArrayLibrary.Array_Add` (`local.TileCheck`) (- (`local.RefeTile`) 10))
  ;[0.05 0.05 0.05] Droite
  (`KismetArrayLibrary.Array_Add` (`local.TileCheck`) (+ (`local.RefeTile`) 20))
  (`KismetArrayLibrary.Array_Add` (`local.TileCheck`) (+ (`local.RefeTile`) 10))
  ;[0.05 0.05 0.05] Devant
  (bind _addtile_ (`self.CheckOwnTile` _returnvalue))
  (if _addtile_
    (`KismetArrayLibrary.Array_Add` (`local.TileCheck`) _returnvalue))
  (bind _addtile__2 (`self.CheckOwnTile` _returnvalue_2))
  (if _addtile__2
    (`KismetArrayLibrary.Array_Add` (`local.TileCheck`) _returnvalue_2))
  (return (`local.TileCheck`)))

(fn `SwitchFar`
  (params (RefTile :type Integer))
  (returns (TileToCheck :type "Array of Integer"))
  (locals (TileCheck :type "Array of Integer") (RefeTile :type Integer))
  (bind _returnvalue (+ (`local.RefeTile`) 2))
  (bind _returnvalue_2 (+ (`local.RefeTile`) 12))
  (bind _returnvalue_3 (+ (`local.RefeTile`) 22))
  (bind _returnvalue_4 (- (`local.RefeTile`) 8))
  (bind _returnvalue_5 (+ (`local.RefeTile`) 21))
  (bind _returnvalue_6 (- (`local.RefeTile`) 19))
  (bind _returnvalue_7 (- (`local.RefeTile`) 18))
  (set `local.RefeTile` RefTile)
  ;[0.05 0.05 0.05] Derriere
  (`KismetArrayLibrary.Array_Add` (`local.TileCheck`) (- (`local.RefeTile`) 2))
  (`KismetArrayLibrary.Array_Add` (`local.TileCheck`) (- (`local.RefeTile`) 12))
  (`KismetArrayLibrary.Array_Add` (`local.TileCheck`) (- (`local.RefeTile`) 22))
  (`KismetArrayLibrary.Array_Add` (`local.TileCheck`) (- (`local.RefeTile`) 21))
  (`KismetArrayLibrary.Array_Add` (`local.TileCheck`) (+ (`local.RefeTile`) 8))
  (`KismetArrayLibrary.Array_Add` (`local.TileCheck`) (+ (`local.RefeTile`) 18))
  (`KismetArrayLibrary.Array_Add` (`local.TileCheck`) (+ (`local.RefeTile`) 19))
  ;[0.05 0.05 0.05] Gauche
  (`KismetArrayLibrary.Array_Add` (`local.TileCheck`) (- (`local.RefeTile`) 20))
  ;[0.05 0.05 0.05] Droite
  (`KismetArrayLibrary.Array_Add` (`local.TileCheck`) (+ (`local.RefeTile`) 20))
  ;[0.05 0.05 0.05] Devant
  (bind _addtile_ (`self.CheckOwnTile` _returnvalue_5))
  (if _addtile_
    (`KismetArrayLibrary.Array_Add` (`local.TileCheck`) _returnvalue_5))
  (bind _addtile__2 (`self.CheckOwnTile` _returnvalue_3))
  (if _addtile__2
    (`KismetArrayLibrary.Array_Add` (`local.TileCheck`) _returnvalue_3))
  (bind _addtile__3 (`self.CheckOwnTile` _returnvalue_2))
  (if _addtile__3
    (`KismetArrayLibrary.Array_Add` (`local.TileCheck`) _returnvalue_2))
  (bind _addtile__4 (`self.CheckOwnTile` _returnvalue))
  (if _addtile__4
    (`KismetArrayLibrary.Array_Add` (`local.TileCheck`) _returnvalue))
  (bind _addtile__5 (`self.CheckOwnTile` _returnvalue_4))
  (if _addtile__5
    (`KismetArrayLibrary.Array_Add` (`local.TileCheck`) _returnvalue_4))
  (bind _addtile__6 (`self.CheckOwnTile` _returnvalue_7))
  (if _addtile__6
    (`KismetArrayLibrary.Array_Add` (`local.TileCheck`) _returnvalue_7))
  (bind _addtile__7 (`self.CheckOwnTile` _returnvalue_6))
  (if _addtile__7
    (`KismetArrayLibrary.Array_Add` (`local.TileCheck`) _returnvalue_6))
  (return (`local.TileCheck`)))

(fn `UserConstructionScript`)