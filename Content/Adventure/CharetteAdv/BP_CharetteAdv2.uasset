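; BP_CharetteAdv2 is the adventure-mode cart (charette) pawn, which travels between adventure tiles and registers itself with BP_TopDownGameMode.
; MoveTo line-traces down to find the current tile, then uses AI MoveTo toward the target while flagging the tile manager as on road.
; On arrival it activates the tile and triggers its next move, also calling the tile's UpdateCharette if the cart actually changed tiles (TimePass).
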(event `self.ReceiveBeginPlay`
  (bind _asbp_top_down_game_mode (cast `/Game/TopDown/Blueprints/BP_TopDownGameMode` (`GameplayStatics.GetGameMode`)))
  (set `self.GM` _asbp_top_down_game_mode)
  (set `/Game/TopDown/Blueprints/BP_TopDownGameMode.CharetteAdv` self (`self.GM`)))

(event `MoveTo`
  (params (TileAdv :type "/Game/Adventure/TilesAdv/BP_TilesAdv Object Reference"))
  (bind _asbp_tiles_adv (`self.OnWhichTile`))
  (`|ExecutionSequence`
    (:`then_0`
      (set `/Game/Adventure/TilesAdv/BP_TileManagerAdv.OnRoad?` true (`/Game/TopDown/Blueprints/BP_TopDownGameMode.TilesManagerAdv` (`self.GM`)))
      (`|AIMoveTo` self (`self.K2_GetActorLocation` TileAdv) null
        (:`OnSuccess`
          (`|ExecutionSequence`
            (:`then_0`
              (`/Game/Adventure/TilesAdv/BP_TilesAdv.ActiveTile` TileAdv)
              (`/Game/Adventure/TilesAdv/BP_TilesAdv.NewMove` TileAdv)
              (set `/Game/Adventure/TilesAdv/BP_TileManagerAdv.OnRoad?` false (`/Game/TopDown/Blueprints/BP_TopDownGameMode.TilesManagerAdv` (`self.GM`))))
            (:`then_1`
              (if (`self.TimePass?`)
                (`/Game/Adventure/TilesAdv/BP_TilesAdv.UpdateCharette` TileAdv)
                (set `self.TimePass?` false)))))))
    (:`then_1`
      (if (!= _asbp_tiles_adv TileAdv)
        (set `self.TimePass?` true)
        (else
          (set `self.TimePass?` false))))))

(fn `OnWhichTile`
  (returns (`AsBP Tiles Adv` :type "/Game/Adventure/TilesAdv/BP_TilesAdv Object Reference"))
  (bind _returnvalue (`self.K2_GetActorLocation`))
  (bind _outhit (`KismetSystemLibrary.LineTraceSingleByProfile` _returnvalue (- _returnvalue (0.0 0.0 150.0)) "BP_TilesAdv"))
  (bind _asbp_tiles_adv (cast `/Game/Adventure/TilesAdv/BP_TilesAdv` (`.HitActor` (`GameplayStatics.BreakHitResult` _outhit))))
  (return _asbp_tiles_adv))

(fn `UserConstructionScript`)