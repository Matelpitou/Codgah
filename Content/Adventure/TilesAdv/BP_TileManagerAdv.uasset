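; BP_TileManagerAdv is the tile manager for Adventure mode, coordinating tile color states.
; On BeginPlay it registers itself as TilesManagerAdv on BP_TopDownGameMode.
; The NewRoad event sets every tile in AllTile to one color state, then applies a second state to the valid tiles in TileAcces.
; Neither array is populated within this Blueprint's graphs.
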(event `self.ReceiveBeginPlay`
  (bind _asbp_top_down_game_mode (cast `/Game/TopDown/Blueprints/BP_TopDownGameMode` (`GameplayStatics.GetGameMode`)))
  (set `self.GM` _asbp_top_down_game_mode)
  (set `/Game/TopDown/Blueprints/BP_TopDownGameMode.TilesManagerAdv` self (`self.GM`)))

(event `NewRoad`
  (for _array_element (`self.AllTile`)
    (`/Game/Adventure/TilesAdv/BP_TilesAdv.ChangeColor` _array_element "NewEnumerator0"))
  (for _array_element_2 (`self.TileAcces`)
    (`/Engine/EditorBlueprintResources/StandardMacros.IsValid` _array_element_2
      (:`Is Valid`
        (`/Game/Adventure/TilesAdv/BP_TilesAdv.ChangeColor` _array_element_2 "NewEnumerator6")))))

(fn `UserConstructionScript`)