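; Clickable adventure-map tile that registers with the game mode's TilesManagerAdv; a Start tile also sets itself as the current tile at play start.
; OnThisTile hands the manager its accessible tiles and triggers NewRoad.
; While not OnRoad, accessible tiles highlight on hover and send CharetteAdv to them on click.
; ChangeColor drives these states through emissive and opacity on a dynamic overlay material.
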(event `self.ReceiveBeginPlay`
  (`KismetSystemLibrary.DelayUntilNextTick`)
  (bind _asbp_top_down_game_mode (cast `/Game/TopDown/Blueprints/BP_TopDownGameMode` (`GameplayStatics.GetGameMode`)))
  (set `self.GM` _asbp_top_down_game_mode)
  (`KismetArrayLibrary.Array_Add` (`/Game/Adventure/TilesAdv/BP_TileManagerAdv.AllTile` (`/Game/TopDown/Blueprints/BP_TopDownGameMode.TilesManagerAdv` (`self.GM`))) self)
  (if (`self.Start?`)
    (`self.OnThisTile`)))

(event `OnThisTile`
  (bind _tilesmanageradv (`/Game/TopDown/Blueprints/BP_TopDownGameMode.TilesManagerAdv` (`self.GM`)))
  (set `/Game/Adventure/TilesAdv/BP_TileManagerAdv.TileActuel` self _tilesmanageradv)
  (set `/Game/Adventure/TilesAdv/BP_TileManagerAdv.TileAcces` (`self.TileAcces`) _tilesmanageradv)
  (`/Game/Adventure/TilesAdv/BP_TileManagerAdv.NewRoad` _tilesmanageradv))

(event `self.Tile.OnClicked`
  (params (TouchedComponent :type "PrimitiveComponent Object Reference") (ButtonPressed :type "Key Structure"))
  ;[0.05 0.05 0.05] On Clicked
  (if (not (`/Game/Adventure/TilesAdv/BP_TileManagerAdv.OnRoad?` (`/Game/TopDown/Blueprints/BP_TopDownGameMode.TilesManagerAdv` (`self.GM`))))
    (for _array_element (`/Game/Adventure/TilesAdv/BP_TileManagerAdv.TileAcces` (`/Game/TopDown/Blueprints/BP_TopDownGameMode.TilesManagerAdv` (`self.GM`)))
      (if (== self _array_element)
        (`/Game/Adventure/CharetteAdv/BP_CharetteAdv2.MoveTo` (`/Game/TopDown/Blueprints/BP_TopDownGameMode.CharetteAdv` (`self.GM`)) self)
        (`self.ChangeColor` "NewEnumerator5")
        (break)))))

(event `self.Tile.OnBeginCursorOver`
  (params (TouchedComponent :type "PrimitiveComponent Object Reference"))
  (if (not (`/Game/Adventure/TilesAdv/BP_TileManagerAdv.OnRoad?` (`/Game/TopDown/Blueprints/BP_TopDownGameMode.TilesManagerAdv` (`self.GM`))))
    (for _array_element (`/Game/Adventure/TilesAdv/BP_TileManagerAdv.TileAcces` (`/Game/TopDown/Blueprints/BP_TopDownGameMode.TilesManagerAdv` (cast `/Game/TopDown/Blueprints/BP_TopDownGameMode` (`GameplayStatics.GetGameMode`) :!pure true)))
      (if (== self _array_element)
        (`self.ChangeColor` "NewEnumerator2")))))

(event `self.Tile.OnEndCursorOver`
  (params (TouchedComponent :type "PrimitiveComponent Object Reference"))
  (if (`/Game/Adventure/TilesAdv/BP_TileManagerAdv.OnRoad?` (`/Game/TopDown/Blueprints/BP_TopDownGameMode.TilesManagerAdv` (`self.GM`)))
    _
    (elif (`|EnumEquality` (`self.ColorTile`) "NewEnumerator2")
      (`self.ChangeColor` "NewEnumerator6"))))

(fn `ChangeColor`
  (params (MatTile :type "/Game/DataTable/Enum/Enum_Tile Enum" :default "NewEnumerator0"))
  (set `self.ColorTile` MatTile)
  (switch `/Game/DataTable/Enum/Enum_Tile` MatTile
    (:`NewEnumerator0`
      (`self.EmissiveTile` (struct)))
    (:`NewEnumerator6`
      (`self.EmissiveTile` (struct :`R` 0.728367 :`G` 1.0 :`B` 0.980086 :`A` 1.0) 1.0 0.15))
    (:`NewEnumerator2`
      (`self.EmissiveTile` (struct :`G` 0.909328 :`B` 1.0 :`A` 1.0) 1.0 0.5))
    (:`NewEnumerator5`
      (`self.EmissiveTile` (struct :`R` 1.0 :`G` 0.992241 :`A` 1.0) 1.0 0.5)))
  (`MeshComponent.SetOverlayMaterial` (`self.Tile`) (`self.MITilesRef`)))

(fn `EmissiveTile`
  (params (Value :type "LinearColor Structure") (Emissive :type "Float (single-precision)") (Opacity :type "Float (single-precision)"))
  (`MaterialInstanceDynamic.SetVectorParameterValue` (`self.MITilesRef`) "EmissiveColor" Value)
  (`MaterialInstanceDynamic.SetScalarParameterValue` (`self.MITilesRef`) "Emissive" Emissive)
  (`MaterialInstanceDynamic.SetScalarParameterValue` (`self.MITilesRef`) "Opacity" Opacity))

(fn `UserConstructionScript`
  (bind _returnvalue (`KismetMaterialLibrary.CreateDynamicMaterialInstance` (`self.MITiles`)))
  (set `self.MITilesRef` _returnvalue))